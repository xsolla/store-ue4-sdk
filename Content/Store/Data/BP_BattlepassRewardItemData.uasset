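; Battle pass reward item data object for the store, holding a reward's name, description, quantity, image URL and icon.
; Getter functions expose each field.
; A RefreshIcon event stores a supplied icon and sets a ready flag, which IsIconSet reports, so the icon can be filled in separately from the other data.
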(event `/Xsolla/Common/Interface/BPI_IconPresenter.RefreshIcon`
  (params (Icon :type "SlateBrush Structure"))
  (set `self.Icon` Icon)
  (set `self.IsIconReady` true))

(fn `GetDescription`
  (returns (Description :type String))
  (return (`self.Description`)))

(fn `GetIcon`
  (returns (Icon :type "SlateBrush Structure"))
  (return (`self.Icon`)))

(fn `GetImageUrl`
  (returns (ImageUrl :type String))
  (return (`self.ImageUrl`)))

(fn `GetName`
  (returns (Name :type String))
  (return (`self.Name`)))

(fn `GetQuantity`
  (returns (Quantity :type Integer))
  (return (`self.Quantity`)))

(fn `IsIconSet`
  (returns (IsIconSet :type Boolean))
  (return (`self.IsIconReady`)))