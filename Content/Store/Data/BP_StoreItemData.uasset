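; BP_StoreItemData is a data wrapper for one store item, exposing its name, SKU, pricing, groups, bundle type, subscription period and cart/purchase state through getters.
; Most getters read the ItemData struct, with real-money prices formatted with their currency.
; GetPriceVC lazily builds and caches a BP_VCPrice object from the first virtual price entry.
; RefreshIcon stores the supplied icon and flags it as ready for IsIconSet.
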(event `/Xsolla/Common/Interface/BPI_IconPresenter.RefreshIcon`
  (params (Icon :type "SlateBrush Structure"))
  (set `self.Icon` Icon)
  (set `self.IsIconReady` true))

(fn `GetBundleType`
  (returns (BundleType :type String))
  (return (`.bundle_type` (break `StoreItem` (`self.ItemData`)))))

(fn `GetDescription`
  (returns (Description :type String))
  (return (`.description` (break `StoreItem` (`self.ItemData`)))))

(fn `GetDisplayPriceRM`
  (returns (Price :type String))
  (bind (_amount _amount_without_discount _currency) (break `StorePrice` (`.price` (break `StoreItem` (`self.ItemData`)))))
  (return (`XsollaStoreLibrary.FormatPrice` (`KismetStringLibrary.Conv_StringToDouble` _amount) _currency)))

(fn `GetDisplayPriceWithoutDiscountRM`
  (returns (Price :type String))
  (bind (_amount _amount_without_discount _currency) (break `StorePrice` (`.price` (break `StoreItem` (`self.ItemData`)))))
  (return (`XsollaStoreLibrary.FormatPrice` (`KismetStringLibrary.Conv_StringToDouble` _amount_without_discount) _currency)))

(fn `GetGroups`
  (returns (Groups :type "Map of String to String"))
  (locals (ItemGroups :type "Map of String to String"))
  (for _array_element (`.groups` (break `StoreItem` (`self.ItemData`)))
    (bind (_id _external_id _name) (break `StoreGroup` _array_element))
    (`BlueprintMapLibrary.Map_Add` (`local.ItemGroups`) _external_id _name))
  (return (`local.ItemGroups`)))

(fn `GetIcon`
  (returns (Icon :type "SlateBrush Structure"))
  (return (`self.Icon`)))

(fn `GetImageUrl`
  (returns (ImageUrl :type String))
  (return (`.image_url` (break `StoreItem` (`self.ItemData`)))))

(fn `GetName`
  (returns (Name :type String))
  (return (`.name` (break `StoreItem` (`self.ItemData`)))))

(fn `GetParent`
  (returns (Parent :type "/Xsolla/Store/Interface/BPI_StorePanel Interface"))
  (return (`self.Parent`)))

(fn `GetPriceVC`
  (returns (Price :type "/Xsolla/Store/Interface/BPI_VCPrice Interface"))
  (bind (_sku _name _description _type _virtual_item_type _groups _is_free _price _virtual_prices) (break `StoreItem` (`self.ItemData`)))
  (bind (_sku_2 _is_default _amount _amount_without_discount _image_url) (break `VirtualCurrencyPrice` (`|GetArrayItem` _virtual_prices)))
  (`/Engine/EditorBlueprintResources/StandardMacros.IsValid` (`self.VCPrice`)
    (:`Is Valid`
      (return (`self.VCPrice`)))
    (:`Is Not Valid`
      (if (> (`KismetArrayLibrary.Array_Length` _virtual_prices) 0)
        (bind _returnvalue (`|GenericCreateObject` "/Xsolla/Store/Data/BP_VCPrice.BP_VCPrice_C" self _sku_2 _amount _amount_without_discount _image_url))
        (bind _output_get (set `self.VCPrice` _returnvalue))
        (return _output_get)))))

(fn `GetSku`
  (returns (Sku :type String))
  (return (`.sku` (break `StoreItem` (`self.ItemData`)))))

(fn `GetSubscriptionDuration`
  (returns (Duration :type Integer))
  (return (`.value` (break `ItemExpirationPeriod` (`.expiration_period` (break `ItemInventoryOptions` (`.inventory_options` (break `StoreItem` (`self.ItemData`)))))))))

(fn `GetSubscriptionDurationType`
  (returns (DurationType :type String))
  (return (`.type` (break `ItemExpirationPeriod` (`.expiration_period` (break `ItemInventoryOptions` (`.inventory_options` (break `StoreItem` (`self.ItemData`)))))))))

(fn `GetVirtualItemType`
  (returns (VirtualItemType :type String))
  (return (`.virtual_item_type` (break `StoreItem` (`self.ItemData`)))))

(fn `IsIconSet`
  (returns (IsIconSet :type Boolean))
  (return (`self.IsIconReady`)))

(fn `IsItemInCart`
  (returns (IsInCart :type Boolean))
  (return (`self.IsInCart`)))

(fn `IsItemPurchased`
  (returns (IsPurchased :type Boolean))
  (return (`self.IsPurchased`)))