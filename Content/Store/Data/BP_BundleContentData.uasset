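; BP_BundleContentData is a store data object that represents one item of content within a bundle.
; Getters expose the name, description, image URL and quantity from its ItemData.
; The icon is held separately: a RefreshIcon event stores it and sets a ready flag, which IsIconSet reports alongside GetIcon.
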(event `/Xsolla/Common/Interface/BPI_IconPresenter.RefreshIcon`
  (params (Icon :type "SlateBrush Structure"))
  (set `self.Icon` Icon)
  (set `self.IsIconReady` true))

(fn `GetDescription`
  (returns (Description :type String))
  (return (`.description` (break `StoreBundleContent` (`self.ItemData`)))))

(fn `GetIcon`
  (returns (Icon :type "SlateBrush Structure"))
  (return (`self.Icon`)))

(fn `GetImageUrl`
  (returns (ImageUrl :type String))
  (return (`.image_url` (break `StoreBundleContent` (`self.ItemData`)))))

(fn `GetName`
  (returns (Name :type String))
  (return (`.name` (break `StoreBundleContent` (`self.ItemData`)))))

(fn `GetQuantity`
  (returns (Quantity :type Integer))
  (return (`.quantity` (break `StoreBundleContent` (`self.ItemData`)))))

(fn `IsIconSet`
  (returns (IsIconSet :type Boolean))
  (return (`self.IsIconReady`)))