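; BP_CartItemData is a data object for one store cart item, exposing its details, parent, icon and real-money prices through getters.
; Display and total prices are currency-formatted, using a quantity-based discount calculation for the default store project and the item's own price amount otherwise.
; A RefreshIcon event stores the supplied icon and flags it as ready, which IsIconSet reports.
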(event `/Xsolla/Common/Interface/BPI_IconPresenter.RefreshIcon`
  (params (Icon :type "SlateBrush Structure"))
  (set `self.Icon` Icon)
  (set `self.IsIconReady` true))

(fn `GetDescription`
  (returns (Description :type String))
  (return (`.description` (break `StoreCartItem` (`self.ItemData`)))))

(fn `GetDisplayPriceRM`
  (returns (Price :type String))
  (bind (_sku _name _attributes _groups _description _long_description _type _virtual_item_type _is_free _price _vc_prices _image_url _quantity) (break `StoreCartItem` (`self.ItemData`)))
  (bind (_amount _amount_without_discount _currency) (break `XsollaPrice` _price))
  (return (`XsollaStoreLibrary.FormatPrice` (select `bool` (`/Xsolla/Store/BP_StoreUtilsMacro.IsDefaultStoreProject`) :`false` (`KismetStringLibrary.Conv_StringToDouble` _amount) :`true` (`/Xsolla/Store/BP_StoreUtilsMacro.Calculate Item Discount` (`KismetStringLibrary.Conv_StringToDouble` _amount_without_discount) _quantity)) _currency)))

(fn `GetDisplayPriceWithoutDiscountRM`
  (returns (Price :type String))
  (bind (_amount _amount_without_discount _currency) (break `XsollaPrice` (`.price` (break `StoreCartItem` (`self.ItemData`)))))
  (return (`XsollaStoreLibrary.FormatPrice` (`KismetStringLibrary.Conv_StringToDouble` _amount_without_discount) _currency)))

(fn `GetIcon`
  (returns (Icon :type "SlateBrush Structure"))
  (return (`self.Icon`)))

(fn `GetImageUrl`
  (returns (ImageUrl :type String))
  (return (`.image_url` (break `StoreCartItem` (`self.ItemData`)))))

(fn `GetIsFree`
  (returns (bIsFree :type Boolean))
  (return (`.is_free` (break `StoreCartItem` (`self.ItemData`)))))

(fn `GetName`
  (returns (Name :type String))
  (return (`.name` (break `StoreCartItem` (`self.ItemData`)))))

(fn `GetParent`
  (returns (Parent :type "/Xsolla/Store/Interface/BPI_CartPanel Interface"))
  (return (`self.Parent`)))

(fn `GetPriceRM`
  (returns (Price :type String))
  (return (`.amount` (break `XsollaPrice` (`.price` (break `StoreCartItem` (`self.ItemData`)))))))

(fn `GetPriceWithoutDiscountRM`
  (returns (Price :type String))
  (return (`.amount_without_discount` (break `XsollaPrice` (`.price` (break `StoreCartItem` (`self.ItemData`)))))))

(fn `GetQuantity`
  (returns (Quantity :type Integer))
  (return (`.quantity` (break `StoreCartItem` (`self.ItemData`)))))

(fn `GetSku`
  (returns (Sku :type String))
  (return (`.sku` (break `StoreCartItem` (`self.ItemData`)))))

(fn `GetTotalPriceRM`
  (returns (Price :type String))
  (bind (_sku _name _attributes _groups _description _long_description _type _virtual_item_type _is_free _price _vc_prices _image_url _quantity) (break `StoreCartItem` (`self.ItemData`)))
  (bind (_amount _amount_without_discount _currency) (break `XsollaPrice` _price))
  (return (`XsollaStoreLibrary.FormatPrice` (* _quantity (select `bool` (`/Xsolla/Store/BP_StoreUtilsMacro.IsDefaultStoreProject`) :`false` (`KismetStringLibrary.Conv_StringToDouble` _amount) :`true` (`/Xsolla/Store/BP_StoreUtilsMacro.Calculate Item Discount` (`KismetStringLibrary.Conv_StringToDouble` _amount_without_discount) _quantity))) _currency)))

(fn `IsIconSet`
  (returns (IsIconSet :type Boolean))
  (return (`self.IsIconReady`)))