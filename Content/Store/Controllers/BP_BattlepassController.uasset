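; BP_BattlepassController drives the battlepass panel in the Xsolla store demo.
; Refreshing shows a loader and updates user attributes through the Xsolla Login subsystem with the current token.
; On success it hides the loader, refreshes the panel and activates it in the demo widget; on failure it hides the loader and shows an error popup.
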(event `/Xsolla/Store/Controllers/BPI_BattlepassController.Init`
  (params (Demo :type "/Xsolla/Login/Interface/BPI_Demo Interface") (DemoWidget :type "/Xsolla/Login/Interface/BPI_DemoWidget Interface"))
  (set `self.Demo` Demo)
  (set `self.DemoWidget` DemoWidget))

(event `/Xsolla/Store/Controllers/BPI_BattlepassController.RefreshBattlepassPanel`
  (params (BattlepassPanel :type "/Xsolla/Store/Interface/BPI_BattlepassPanel Interface"))
  (`/Xsolla/Common/BP_DemoUtils.ShowLoader` true)
  (`XsollaLoginSubsystem.UpdateUserAttributes` :`self` (subsystem `XsollaLoginSubsystem`) :`AuthToken` (`/Xsolla/Login/Misc/BP_TokenUtils.GetToken`) :`SuccessCallback` (delegate `OnUserAttributesReceived`) :`ErrorCallback` (delegate `UpdateUserAttributesError`)))

(event `OnUserAttributesReceived`
  (`/Xsolla/Common/BP_DemoUtils.ShowLoader` false)
  (`/Xsolla/Store/Interface/BPI_BattlepassPanel.RefreshPanel` (stale `/Xsolla/Store/Controllers/BPI_BattlepassController.RefreshBattlepassPanel` BattlepassPanel))
  (`/Xsolla/Login/Interface/BPI_DemoWidget.ActivateBattlepassPanel` (`self.DemoWidget`)))

(event `UpdateUserAttributesError`
  (params (Code :type String) (Description :type String))
  (`/Xsolla/Common/BP_DemoUtils.ShowLoader` false)
  (`/Xsolla/Common/BP_DemoUtils.ShowMessagePopup` (`KismetTextLibrary.Conv_StringToText` Description) true))