(event `/Xsolla/Store/Controllers/BPI_StoreController.OnBundlePreviewOpenInitiated`
  (params (Sku :type String) (StorePanel :type "/Xsolla/Store/Interface/BPI_StorePanel Interface"))
  ;[1 1 1] Open Preview Bundle
  (`/Xsolla/Common/BP_DemoUtils.ShowLoader` true)
  (`XsollaStoreSubsystem.GetSpecifiedBundle` (subsystem `XsollaStoreSubsystem`) Sku (delegate `OnGetSpecifiedBundleSuccess`) (`|CreateDelegate` :!event `ShowStoreError`)))

(event `OnGetSpecifiedBundleSuccess`
  (params (Bundle :type "StoreBundle Structure"))
  ;[1 1 1] Open Preview Bundle
  (`/Xsolla/Common/BP_DemoUtils.ShowLoader` false)
  (bind (_bundleitemdata _bundlecontent) (`self.CreateBundleData` Bundle))
  (bind _returnvalue (`|CreateWidget` "/Xsolla/Store/Popup/W_PreviewBundlePopup.W_PreviewBundlePopup_C" (`GameplayStatics.GetPlayerController` 0) _bundleitemdata _bundlecontent (stale `/Xsolla/Store/Controllers/BPI_StoreController.OnBundlePreviewOpenInitiated` StorePanel)))
  (`UserWidget.AddToViewport` _returnvalue 10000))

(event `/Xsolla/Store/Controllers/BPI_StoreController.RefreshStorePanel`
  (params (ActivateWhenReady :type Boolean) (StorePanel :type "/Xsolla/Store/Interface/BPI_StorePanel Interface"))
  ;[1 1 1] Refresh store panel
  (bind _storedata (`self.CreateStoreData` StorePanel))
  (`/Xsolla/Store/Interface/BPI_StorePanel.RefreshStoreItemsList` StorePanel _storedata)
  (if ActivateWhenReady
    (`/Xsolla/Login/Interface/BPI_DemoWidget.ActivateStorePanel` (`self.DemoWidget`))))

(event `/Xsolla/Store/Controllers/BPI_StoreController.RefreshCurrencyPanel`
  (params (ActivateWhenReady :type Boolean) (CurrencyPanel :type "/Xsolla/Store/Interface/BPI_StorePanel Interface"))
  ;[1 1 1] Refresh store panel
  (bind _storedata (`self.CreateCurrencyData` CurrencyPanel))
  (`/Xsolla/Store/Interface/BPI_StorePanel.RefreshStoreItemsList` CurrencyPanel _storedata)
  (if ActivateWhenReady
    (`/Xsolla/Login/Interface/BPI_DemoWidget.ActivateCurrencyPanel` (`self.DemoWidget`))))

(event `Init`
  (params (InDemo :type "/Xsolla/Login/Interface/BPI_Demo Interface") (InDemoWidget :type "/Xsolla/Login/Interface/BPI_DemoWidget Interface") (InInventoryController :type "/Xsolla/Inventory/Controllers/BPI_InventoryController Interface"))
  ;[1 1 1] Init
  (set `self.Demo` InDemo)
  (set `self.DemoWidget` InDemoWidget)
  (set `self.Inventory Controller` InInventoryController)
  (`XsollaStoreSubsystem.Initialize` (subsystem `XsollaStoreSubsystem`) (select `bool` (`/Xsolla/Common/BP_DemoUtils.Does Dev Menu Save Game Exist`) :`false` (`XsollaProjectSettings.ProjectID` (`XsollaSettingsLibrary.GetProjectSettings`)) :`true` (`.ProjectID_10_F159CBC8422282C5B7D45F8672FE9D4F` (break `/Xsolla/Common/Misc/XsollaDevMenuData` (`/Xsolla/Common/BP_DemoUtils.LoadDevMenuData`)))))
  (`/Xsolla/Common/BP_DemoUtils.ShowLoader` true)
  (`XsollaStoreSubsystem.UpdateVirtualItems` :`self` (subsystem `XsollaStoreSubsystem`) :`AdditionalFields` (`|MakeArray` "long_description") :`SuccessCallback` (delegate `OnVirtualItemsUpdateSuccess`))
  (`XsollaStoreSubsystem.UpdateVirtualCurrencies` :`self` (subsystem `XsollaStoreSubsystem`) :`SuccessCallback` (delegate `OnUpdateVirtualCurrenciesSuccess`))
  (`XsollaStoreSubsystem.UpdateVirtualCurrencyPackages` :`self` (subsystem `XsollaStoreSubsystem`) :`AdditionalFields` (`|MakeArray` "long_description") :`SuccessCallback` (delegate `OnUpdateVCPackagesSuccess`)))

(event `OnVirtualItemsUpdateSuccess`
  ;[1 1 1] Init
  (set `self.StoreReady` true)
  ;;[1 1 1] Fix race condition
  (`XsollaStoreSubsystem.GetBundles` :`self` (subsystem `XsollaStoreSubsystem`) :`SuccessCallback` (delegate `OnGetListOfBundlesSuccess`) :`ErrorCallback` (delegate `OnGetListOfBundlesFailed`)))

(event `OnUpdateVirtualCurrenciesSuccess`
  (params (VirtualCurrencyData :type "VirtualCurrencyData Structure (by ref)"))
  ;[1 1 1] Init
  (set `self.VCReady` true)
  (if (and (`self.StoreReady`) (`self.VCReady`) (`self.VCPackagesReady`) (`self.bIsBundlesReady`)) :!label _label
    (`/Xsolla/Common/BP_DemoUtils.ShowLoader` false)))

(event `OnUpdateVCPackagesSuccess`
  ;[1 1 1] Init
  (set `self.VCPackagesReady` true)
  (goto _label))

(event `OnGetListOfBundlesSuccess`
  (params (ListOfBundles :type "StoreListOfBundles Structure"))
  ;[1 1 1] Init
  ;;[1 1 1] Fix race condition
  (set `self.bIsBundlesReady` true :!label _label_2)
  (goto _label))

(event `OnGetListOfBundlesFailed`
  (params (StatusCode :type Integer) (ErrorCode :type Integer) (ErrorMessage :type String))
  ;[1 1 1] Init
  ;;[1 1 1] Fix race condition
  (goto _label_2))

(fn `CreateBundleData`
  (params (ItemData :type "StoreBundle Structure"))
  (returns (BundleItemData :type "/Xsolla/Store/Interface/BPI_BundleItemData Interface") (BundleContent :type "Array of /Xsolla/Store/Interface/BPI_BundleContentItemData Interface"))
  (locals (IconPresenters :type "Array of /Xsolla/Common/Interface/BPI_IconPresenter Interface") (LocalBundleContent :type "Array of /Xsolla/Store/Interface/BPI_BundleContentItemData Interface"))
  (bind _returnvalue (`|GenericCreateObject` "/Xsolla/Store/Data/BP_BundleItemData.BP_BundleItemData_C" (`GameplayStatics.GetPlayerController` 0) ItemData))
  (`KismetArrayLibrary.Array_Add` (`local.IconPresenters`) _returnvalue)
  (bind _price (`/Xsolla/Store/Interface/BPI_BundleItemData.GetPriceVC` _returnvalue))
  (bind _asbp_vcprice (cast `/Xsolla/Store/Data/BP_VCPrice` _price)
    (:`then`
      (`KismetArrayLibrary.Array_Add` (`local.IconPresenters`) _asbp_vcprice))
    (:`CastFailed`
      _))
  (bind _content (`/Xsolla/Store/Interface/BPI_BundleItemData.GetContent` _returnvalue))
  (for _array_element _content
    (bind _returnvalue_2 (`|GenericCreateObject` "/Xsolla/Store/Data/BP_BundleContentData.BP_BundleContentData_C" (`GameplayStatics.GetPlayerController` 0) _array_element))
    (`KismetArrayLibrary.Array_Add` (`local.LocalBundleContent`) _returnvalue_2)
    (`KismetArrayLibrary.Array_Add` (`local.IconPresenters`) _returnvalue_2))
  (bind _iconsloader (`/Xsolla/Login/Interface/BPI_Demo.GetIconsLoader` (`self.Demo`)))
  (`/Xsolla/Login/Interface/BPI_IconsLoader.LoadIcons` _iconsloader (`local.IconPresenters`))
  (return _returnvalue (`local.LocalBundleContent`)))

(fn `CreateCurrencyData`
  (params (Store :type "/Xsolla/Store/Interface/BPI_StorePanel Interface"))
  (returns (StoreData :type "Array of /Xsolla/Store/Interface/BPI_StoreItemData Interface"))
  (locals (StoreItemData :type "Array of /Xsolla/Store/Interface/BPI_StoreItemData Interface") (IconPresenters :type "Array of /Xsolla/Common/Interface/BPI_IconPresenter Interface"))
  (for _array_element (`XsollaStoreSubsystem.GetVirtualCurrencyPackages` (subsystem `XsollaStoreSubsystem`))
    (bind _returnvalue (`|GenericCreateObject` "/Xsolla/Store/Data/BP_CurrencyPackageItemData.BP_CurrencyPackageItemData_C" (`GameplayStatics.GetPlayerController` 0) _array_element Store))
    (`KismetArrayLibrary.Array_Add` (`local.StoreItemData`) _returnvalue)
    (`KismetArrayLibrary.Array_Add` (`local.IconPresenters`) _returnvalue)
    (bind _price (`/Xsolla/Store/Data/BP_StoreItemData.GetPriceVC` _returnvalue))
    (bind _asbp_vcprice (cast `/Xsolla/Store/Data/BP_VCPrice` _price))
    (`KismetArrayLibrary.Array_Add` (`local.IconPresenters`) _asbp_vcprice))
  (bind _iconsloader (`/Xsolla/Login/Interface/BPI_Demo.GetIconsLoader` (`self.Demo`)))
  (`/Xsolla/Login/Interface/BPI_IconsLoader.LoadIcons` _iconsloader (`local.IconPresenters`))
  (return (`local.StoreItemData`)))

(fn `CreateStoreData`
  (params (Store :type "/Xsolla/Store/Interface/BPI_StorePanel Interface"))
  (returns (StoreData :type "Array of /Xsolla/Store/Interface/BPI_StoreItemData Interface"))
  (locals (StoreItemData :type "Array of /Xsolla/Store/Interface/BPI_StoreItemData Interface") (IconPresenters :type "Array of /Xsolla/Common/Interface/BPI_IconPresenter Interface"))
  (bind _returnvalue_items (break `StoreItemsData` (`XsollaStoreSubsystem.GetItemsData` (subsystem `XsollaStoreSubsystem`))))
  (for _array_element _returnvalue_items
    (bind ((`sku` _sku) (`virtual_item_type` _virtual_item_type)) (break `StoreItem` _array_element))
    (bind _isininventory (`/Xsolla/Inventory/Controllers/BPI_InventoryController.IsItemInInventory` (`self.Inventory Controller`) _sku))
    (bind _returnvalue (`|GenericCreateObject` "/Xsolla/Store/Data/BP_StoreItemData.BP_StoreItemData_C" (`GameplayStatics.GetPlayerController` 0) _array_element Store (and _isininventory (`KismetStringLibrary.EqualEqual_StrStr` _virtual_item_type "non_consumable"))))
    (`KismetArrayLibrary.Array_Add` (`local.StoreItemData`) _returnvalue)
    (`KismetArrayLibrary.Array_Add` (`local.IconPresenters`) _returnvalue)
    (bind _price (`/Xsolla/Store/Data/BP_StoreItemData.GetPriceVC` _returnvalue))
    (bind _asbp_vcprice (cast `/Xsolla/Store/Data/BP_VCPrice` _price))
    (`KismetArrayLibrary.Array_Add` (`local.IconPresenters`) _asbp_vcprice))
  (bind _iconsloader (`/Xsolla/Login/Interface/BPI_Demo.GetIconsLoader` (`self.Demo`)))
  (`/Xsolla/Login/Interface/BPI_IconsLoader.LoadIcons` _iconsloader (`local.IconPresenters`))
  (return (`local.StoreItemData`)))

(fn `ShowStoreError`
  (params (StatusCode :type Integer) (ErrorCode :type Integer) (ErrorMessage :type String))
  (`/Xsolla/Common/BP_DemoUtils.ShowLoader` false)
  (`/Xsolla/Common/BP_DemoUtils.ShowMessagePopup` (`KismetTextLibrary.Conv_StringToText` ErrorMessage) true))