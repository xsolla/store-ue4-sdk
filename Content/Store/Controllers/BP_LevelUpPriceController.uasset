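; Store demo controller that supplies the level-up price panel with virtual currency data from the Xsolla store subsystem.
; On refresh it builds a price data object from a currency's SKU and image URL, has the demo load its icon, then passes it to the panel.
; The default store project uses the "gold" currency, while other projects take the first currency available.
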(event `/Xsolla/Store/Controllers/BPI_LevelUpPriceController.RefreshLevelUpPricePanel`
  (params (Panel :type "/Xsolla/Store/Interface/BPI_LevelUpPricePresenter Interface"))
  ;[1 1 1] refresh levelup price panel
  (bind _levelupprice (`self.CreateLevelUpPriceData`))
  (`/Xsolla/Store/Interface/BPI_LevelUpPricePresenter.RefreshLevelUpPriceData` Panel _levelupprice))

(fn `CreateLevelUpPriceData`
  (returns (LevelUpPrice :type "/Xsolla/Common/Data/BP_LevelUpPriceData Object Reference"))
  (for _array_element (`XsollaStoreSubsystem.GetVirtualCurrencyData` (subsystem `XsollaStoreSubsystem`))
    (if (`/Xsolla/Store/BP_StoreUtilsMacro.IsDefaultStoreProject`)
      (bind (_sku _name _groups _attributes _type _description _image_url) (break `VirtualCurrency` _array_element))
      (if (`KismetStringLibrary.EqualEqual_StrStr` _sku "gold")
        (bind _returnvalue (`|GenericCreateObject` "/Xsolla/Common/Data/BP_LevelUpPriceData.BP_LevelUpPriceData_C" self _sku _image_url :!label _label))
        (`/Xsolla/Login/Interface/BPI_Demo.LoadIcons` (`self.Demo`) (`|MakeArray` _returnvalue :!type "/Xsolla/Common/Interface/BPI_IconPresenter Interface"))
        (return _returnvalue))
      (else
        (goto _label))))
  (return null))

(fn `Init`
  (params (InDemo :type "/Xsolla/Login/Interface/BPI_Demo Interface") (InDemoWidget :type "/Xsolla/Login/Interface/BPI_DemoWidget Interface"))
  (set `self.Demo` InDemo)
  (set `self.DemoWidget` InDemoWidget))