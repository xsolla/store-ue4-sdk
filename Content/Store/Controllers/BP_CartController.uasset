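; Cart controller for the Xsolla store demo that handles refreshing, adding, removing, clearing and promocode redemption through the store subsystem.
; It builds item data and locally calculated prices from the cached cart to feed the cart panel and counter.
; Add and remove update the UI immediately, restart a delayed refresh timer and resync on error.
; Promocodes persist in a save slot, and bonus-only carts are cleared with a popup.
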(event Custom|OnEmptyCartWithBonusPopupResult
  (params (IsConfirmed :type Boolean))
  ;[1 1 1] Refresh cart panel using local cache
  (Default|CloseCart (Variables|Default|GetDemoWidget)))

(event Custom|OnEmptyCartWithBonusClearSuccess
  ;[1 1 1] Refresh cart panel using local cache
  (CallFunction|RefreshCartCounter)
  (CallFunction|UpdateCartPromocode))

(event Custom|OnUpdateCartSuccess
  ;[1 1 1] Refresh cart panel
  (CallFunction|ShowLoader false)
  (bind _cartdata (CallFunction|CreateCartData (stale EventRefreshCartPanel CartPanel)))
  (bind (_cartprice _discount _cartpricewithoutdiscount) (CallFunction|CalculateCartPrice _cartdata))
  (Default|RefreshCartItemsList (stale EventRefreshCartPanel CartPanel) _cartdata _cartprice _discount _cartpricewithoutdiscount (CallFunction|GetCartPromocode) (stale EventRefreshCartPanel ActivateWhenReady) (CallFunction|GetCartPromocodeDiscount))
  (if (Variables|Default|GetbNeedOpenCartPanel)
    (Default|ActivateCartPanel (Variables|Default|GetDemoWidget))
    (Variables|Default|SetbNeedOpenCartPanel false)))

(event Custom|OnRedeemPromocodeSuccess
  ;[1 1 1] Redeem promocode
  (CallFunction|ShowLoader false)
  (CallFunction|UpdateCartPromocode (stale EventOnRedeemPromocodeInitiated Promocode))
  (bind _cartdata (CallFunction|CreateCartData (stale EventOnRedeemPromocodeInitiated CartPanel)))
  (bind (_cartprice _discount _cartpricewithoutdiscount) (CallFunction|CalculateCartPrice _cartdata))
  (Default|RefreshCartItemsList (stale EventOnRedeemPromocodeInitiated CartPanel) _cartdata _cartprice _discount _cartpricewithoutdiscount (CallFunction|GetCartPromocode) false (CallFunction|GetCartPromocodeDiscount)))

(event Custom|OnRefreshCartPanelJob
  ;[1 1 1] Refresh Cart Job
  (if (not (Variables|Default|GetbNeedOpenCartPanel)) ; This branch need for disallow race between ActivateWhenReady.\nWhen here is no branch - then call "Open Cart Panel" can happen without ActivateWhenReady.\nWhy it is not only in RefreshCartPanel - because it disable delay between finished Loader and moment of opening of Cart.
    (Default|OnRefreshCartPanelJobFired (Variables|Default|GetDemo))))

(event Custom|OnAddToCartSuccess
  ;[1 1 1] Add/Remove cart items
)

(event Custom|OnAddToCartError
  (params (StatusCode :type Integer) (ErrorCode :type Integer) (ErrorMessage :type String))
  ;[1 1 1] Add/Remove cart items
  (Default|RefreshStorePanelFired (Variables|Default|GetDemo))
  (CallFunction|RefreshCartCounter)
  (CallFunction|RefreshCartPanel false false (stale EventOnAddItemtoCartInitiated CartPanel)))

(event Custom|OnRemoveFromCartSuccess
  ;[1 1 1] Add/Remove cart items
)

(event Custom|OnRemoveFromCartError
  (params (StatusCode :type Integer) (ErrorCode :type Integer) (ErrorMessage :type String))
  ;[1 1 1] Add/Remove cart items
  (Default|RefreshStorePanelFired (Variables|Default|GetDemo))
  (CallFunction|RefreshCartCounter)
  (CallFunction|RefreshCartPanel false false (stale EventOnRemoveItemfromCartInitiated CartPanel)))

(event Custom|OnRedeemPromocodeFailed
  (params (StatusCode :type Integer) (ErrorCode :type Integer) (ErrorMessage :type String))
  ;[1 1 1] Redeem promocode
  (CallFunction|ShowLoader false)
  (if (and (== StatusCode 404) (== ErrorCode 9807))
    (Default|ShowPromocodeError (stale EventOnRedeemPromocodeInitiated CartPanel))
    (else
      (CallFunction|ShowStoreError StatusCode ErrorCode ErrorMessage))))

(event Custom|OnCartClearCommandSuccess
  ;[1 1 1] on cart clear initiated
  (CallFunction|ShowLoader false)
  (CallFunction|RefreshCartPanelWithoutUpdate false (stale EventOnCartClearInitiated CartPanel))
  (CallFunction|RefreshCartCounter)
  (CallFunction|UpdateCartPromocode)
  (if (stale EventOnCartClearInitiated CloseCartWhenReady)
    (Default|CloseCart (Variables|Default|GetDemoWidget))))

(event Custom|OnUpdateCartFailed
  (params (StatusCode :type Integer) (ErrorCode :type Integer) (ErrorMessage :type String))
  ;[1 1 1] Refresh cart panel
  (Variables|Default|SetbNeedOpenCartPanel false)
  (CallFunction|ShowStoreError StatusCode ErrorCode ErrorMessage))

(event EventRefreshCartPanel
  (params (ActivateWhenReady :type Boolean) (bIsSeemlessRefresh :type Boolean) (CartPanel :type BPI%20Cart%20Panel%20Interface))
  ;[1 1 1] Refresh cart panel
  (Variables|Default|SetbNeedOpenCartPanel (or (Variables|Default|GetbNeedOpenCartPanel) ActivateWhenReady))
  (CallFunction|ShowLoader (not bIsSeemlessRefresh))
  (Class|XsollaStoreSubsystem|UpdateCart (Subsystems|GetXsollaStoreSubsystem) (CallFunction|GetToken) "" "" "" (delegate Custom|OnUpdateCartSuccess) (delegate Custom|OnUpdateCartFailed)))

(event EventRefreshCartPanelWithoutUpdate
  (params (ActivateWhenReady :type Boolean) (CartPanel :type BPI%20Cart%20Panel%20Interface))
  ;[1 1 1] Refresh cart panel using local cache
  (bind _cartdata (CallFunction|CreateCartData CartPanel))
  (bind (_cartprice _discount _cartpricewithoutdiscount) (CallFunction|CalculateCartPrice _cartdata))
  (Default|RefreshCartItemsList CartPanel _cartdata _cartprice _discount _cartpricewithoutdiscount (CallFunction|GetCartPromocode) false (CallFunction|GetCartPromocodeDiscount))
  (if (not (CallFunction|IsCartOnlywithBonuses))
    (Utilities|FlowControl|Sequence
      (:then_0
        (if (== (Utilities|Array|Length _cartdata) 0)
          (CallFunction|UpdateCartPromocode)))
      (:then_1
        (if ActivateWhenReady
          (Default|ActivateCartPanel (Variables|Default|GetDemoWidget)))))
    (else
      (bind _returnvalue (UserInterface|CreateWidget "/Xsolla/Common/Popup/W_ConfirmPopup.W_ConfirmPopup_C" (Game|GetPlayerController 0) "You can get the bonus item only if you have at least 1 paid item in the cart." "CONFIRM" true))
      (UserInterface|Viewport|AddtoViewport _returnvalue 10000)
      (EventDispatchers|BindEventtoOnPopupResult _returnvalue (delegate Custom|OnEmptyCartWithBonusPopupResult))
      (Class|XsollaStoreSubsystem|ClearCart (Subsystems|GetXsollaStoreSubsystem) (CallFunction|GetToken) "" (delegate Custom|OnEmptyCartWithBonusClearSuccess) (EventDispatchers|CreateEvent :!event ShowStoreError)))))

(event EventOnCartClearInitiated
  (params (CloseCartWhenReady :type Boolean) (CartPanel :type BPI%20Cart%20Panel%20Interface))
  ;[1 1 1] on cart clear initiated
  (CallFunction|ShowLoader true)
  (Class|XsollaStoreSubsystem|ClearCart (Subsystems|GetXsollaStoreSubsystem) (CallFunction|GetToken) "" (delegate Custom|OnCartClearCommandSuccess) (EventDispatchers|CreateEvent :!event ShowStoreError)))

(event EventOnAddItemtoCartInitiated
  (params (sku :type String) (Quantity :type Integer) (CartPanel :type BPI%20Cart%20Panel%20Interface))
  ;[1 1 1] Add/Remove cart items
  (Class|XsollaStoreSubsystem|AddtoCart (Subsystems|GetXsollaStoreSubsystem) (CallFunction|GetToken) "" sku Quantity (delegate Custom|OnAddToCartSuccess) (delegate Custom|OnAddToCartError))
  (CallFunction|RefreshCartCounter)
  (CallFunction|RefreshCartPanelWithoutUpdate false CartPanel)
  (CallFunction|RunTimerRefreshCart))

(event EventOnRemoveItemfromCartInitiated
  (params (sku :type String) (CartPanel :type BPI%20Cart%20Panel%20Interface))
  ;[1 1 1] Add/Remove cart items
  (Class|XsollaStoreSubsystem|RemovefromCart (Subsystems|GetXsollaStoreSubsystem) (CallFunction|GetToken) "" sku (delegate Custom|OnRemoveFromCartSuccess) (delegate Custom|OnRemoveFromCartError))
  (CallFunction|RefreshCartCounter)
  (CallFunction|RefreshCartPanelWithoutUpdate false CartPanel)
  (CallFunction|RunTimerRefreshCart))

(event EventOnRedeemPromocodeInitiated
  (params (Promocode :type String) (CartPanel :type BPI%20Cart%20Panel%20Interface))
  ;[1 1 1] Redeem promocode
  (CallFunction|ShowLoader true)
  (Class|XsollaStoreSubsystem|RedeemPromocode (Subsystems|GetXsollaStoreSubsystem) (CallFunction|GetToken) Promocode (delegate Custom|OnRedeemPromocodeSuccess) (delegate Custom|OnRedeemPromocodeFailed)))

(fn Init
  (params (InDemo :type BPI%20Demo%20Interface) (InDemoWidget :type BPI%20Demo%20Widget%20Interface))
  (Variables|Default|SetDemo InDemo)
  (Variables|Default|SetDemoWidget InDemoWidget))

(fn GetToken
  (return (Utilities|Struct|BreakXsollaAuthToken (Utilities|Struct|BreakXsollaLoginData (Class|XsollaLoginSubsystem|GetLoginData (Subsystems|GetXsollaLoginSubsystem))))))

(fn ShowStoreError
  (params (StatusCode :type Integer) (ErrorCode :type Integer) (ErrorMessage :type String))
  (CallFunction|ShowLoader false)
  (CallFunction|ShowMessagePopup (Utilities|Text|ToText(String) ErrorMessage) true))

(fn CreateCartData
  (params (Cart :type BPI%20Cart%20Panel%20Interface))
  (for _array_element (.Items (Utilities|Struct|BreakStoreCart (Class|XsollaStoreSubsystem|GetCart (Subsystems|GetXsollaStoreSubsystem))))
    (bind _returnvalue (Game|ConstructObjectfromClass "/Xsolla/Store/Data/BP_CartItemData.BP_CartItemData_C" (Game|GetPlayerController 0) _array_element Cart))
    (Utilities|Array|Add (LocalVariables|GetCartItemData) _returnvalue)
    (Utilities|Array|Add (LocalVariables|GetIconPresenters) _returnvalue))
  (Default|LoadIcons (Variables|Default|GetDemo) (LocalVariables|GetIconPresenters))
  (return (LocalVariables|GetCartItemData)))

(fn CalculateCartPrice
  (params (CartData :type Array%20of%20BPI%20Cart%20Item%20Data%20Interfaces))
  (bind _currency (CallFunction|GetCartCurrency))
  (for _array_element CartData
    (bind _quantity (Default|GetQuantity _array_element))
    (bind _price (Default|GetPriceRM _array_element))
    (bind _price_2 (Default|GetPriceWithoutDiscountRM _array_element))
    (bind _output_get (LocalVariables|SetLocal%20Item%20Price%20No%20Discount (* _quantity (Math|Conversions|ToFloat(Integer) _price_2))))
    (LocalVariables|SetLocal%20Total%20Price (+ (LocalVariables|GetLocal%20Total%20Price) (LocalVariables|GetLocal%20Item%20Price%20No%20Discount)))
    ;[1 1 1] Discount calculation (valid only for demo project 44056)
    (LocalVariables|SetLocal%20Total%20Price%20With%20Discount (+ (LocalVariables|GetLocal%20Total%20Price%20With%20Discount) (select (Utilities|IsDefaultStoreProject) (Utilities|CalculateItemDiscount (LocalVariables|GetLocal%20Item%20Price%20No%20Discount) _quantity) (select (Utilities|Enum|NotEqual(Enum) _price_2 _price) (* _quantity (Math|Conversions|ToFloat(Integer) _price)) _output_get)))))
  (return (Class|XsollaStoreLibrary|FormatPrice (- (LocalVariables|GetLocal%20Total%20Price%20With%20Discount) (|(Price*(percent/100)) (CallFunction|GetCartPromocodeDiscount) (LocalVariables|GetLocal%20Total%20Price%20With%20Discount))) _currency) (Class|XsollaStoreLibrary|FormatPrice (|(Price*(percent/100)) (CallFunction|GetCartPromocodeDiscount) (LocalVariables|GetLocal%20Total%20Price%20With%20Discount)) _currency) (Class|XsollaStoreLibrary|FormatPrice (LocalVariables|GetLocal%20Total%20Price%20With%20Discount) _currency)))

(fn GetCartPromocode
  (bind _returnvalue (SaveGame|LoadGamefromSlot "CartPromocode"))
  (bind _asbp_cart_promocode_data (Utilities|Casting|CastToBP_CartPromocodeData _returnvalue)
    (:then
      (return (Variables|/Xsolla/Login/Data/BP_CartPromocodeData.BP_CartPromocodeData_C|GetPromocode _asbp_cart_promocode_data)))
    (:CastFailed
      (return ""))))

(fn GetCartPromocodeDiscount
  (bind _returnvalue (Subsystems|GetXsollaStoreSubsystem))
  (bind _returnvalue_2 (Class|XsollaStoreSubsystem|GetCart _returnvalue))
  (bind _price (Utilities|Struct|BreakStoreCart _returnvalue_2))
  (bind (_amount _amount_without_discount) (Utilities|Struct|BreakXsollaPrice _price))
  (bind _returnvalue_3 (Math|Conversions|ToFloat(Integer) _amount_without_discount))
  (if (and (Utilities|Array|IsEmpty _amount) (Utilities|Array|IsEmpty _amount_without_discount))
    (return 0.0)
    (else
      (return (|((1.000000-((price-discount)/price))*100) _returnvalue_3 (- _returnvalue_3 (Math|Conversions|ToFloat(Integer) _amount)))))))

(fn GetCartCurrency
  (bind _returnvalue (Subsystems|GetXsollaStoreSubsystem))
  (bind _returnvalue_2 (Class|XsollaStoreSubsystem|GetCart _returnvalue))
  (bind (_cart_id _price _is_free _items) (Utilities|Struct|BreakStoreCart _returnvalue_2))
  (bind _currency (Utilities|Struct|BreakXsollaPrice _price))
  (if (Utilities|Array|IsEmpty _currency)
    (if (> (Utilities|Array|Length _items) 0)
      (return (.currency (Utilities|Struct|BreakXsollaPrice (.price (Utilities|Struct|BreakStoreCartItem (Utilities|Array|Get(acopy) _items)))))) ; Pick first cart entry currency (occur when adding item to empty cart before sync with backend finished)
      (else
        (return "") ; Should occur only when cart is empty
      ))
    (else
      (return _currency))))

(fn UpdateCartPromocode
  (params (Promocode :type String))
  (bind _returnvalue (SaveGame|LoadGamefromSlot "CartPromocode"))
  (bind _asbp_cart_promocode_data (Utilities|Casting|CastToBP_CartPromocodeData _returnvalue)
    (:then
      (Variables|/Xsolla/Login/Data/BP_CartPromocodeData.BP_CartPromocodeData_C|SetPromocode _asbp_cart_promocode_data Promocode)
      (SaveGame|SaveGametoSlot _asbp_cart_promocode_data "CartPromocode"))
    (:CastFailed
      (bind _returnvalue_2 (SaveGame|CreateSaveGameObject "/Xsolla/Login/Data/BP_CartPromocodeData.BP_CartPromocodeData_C"))
      (Variables|/Xsolla/Login/Data/BP_CartPromocodeData.BP_CartPromocodeData_C|SetPromocode _returnvalue_2 Promocode)
      (SaveGame|SaveGametoSlot _returnvalue_2 "CartPromocode"))))

(fn IsCartOnlywithBonuses
  (bind _returnvalue (Subsystems|GetXsollaStoreSubsystem))
  (bind _returnvalue_2 (Class|XsollaStoreSubsystem|GetCart _returnvalue))
  (bind _items (Utilities|Struct|BreakStoreCart _returnvalue_2))
  (for _array_element _items
    (if (not (Utilities|Struct|BreakStoreCartItem _array_element))
      (return false)))
  (return (> (Utilities|Array|Length _items) 0)))

(fn RefreshCartCounter
  (for _array_element (.items (Class|XsollaStoreSubsystem|GetCart (Subsystems|GetXsollaStoreSubsystem)))
    (LocalVariables|SetCartCounter (+ (LocalVariables|GetCartCounter) (.quantity (Utilities|Struct|BreakStoreCartItem _array_element)))))
  (Default|RefreshCartCounter (Variables|Default|GetDemoWidget) (LocalVariables|GetCartCounter)))

(fn RunTimerRefreshCart
  (Utilities|Time|ClearandInvalidateTimerbyHandle (Variables|Default|GetRefreshCartPanelJob))
  (bind _returnvalue (Utilities|Time|SetTimerbyEvent (EventDispatchers|CreateEvent :!event Custom|OnRefreshCartPanelJob) (LocalVariables|GetRefreshCartPanelTime)))
  (Variables|Default|SetRefreshCartPanelJob _returnvalue))