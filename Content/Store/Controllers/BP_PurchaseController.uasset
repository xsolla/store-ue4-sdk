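; Purchase controller for the Xsolla store that handles item and cart purchases with real money, plus item purchases with virtual currency.
; Real-money flows fetch a payment token and open the payment console; cart purchases first verify the cached cart matches the server's.
; Order checks start immediately for platform browsers or virtual currency, otherwise on browser close.
; Order-check objects report status to the result handler, falling back to timed short polling on error or timeout.
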(event `self.LaunchPaymentConsole`
  (params (AccessToken1 :type String) (OrderId1 :type Integer) (ResultHandler :type "/Xsolla/Store/Handlers/BPI_PurchaseResultHandler Interface"))
  ;[1 1 1] Launch payment console
  (bind _browserwidget (`XsollaStoreSubsystem.LaunchPaymentConsole` (subsystem `XsollaStoreSubsystem`) AccessToken1))
  (if (`XsollaStoreSettings.UsePlatformBrowser` (`XsollaStoreLibrary.GetStoreSettings`))
    (`self.Check Pending Order` OrderId1 ResultHandler)
    (else
      (bind _asw_store_browser (cast `/Xsolla/Store/Components/W_StoreBrowser` _browserwidget))
      (add `/Xsolla/Store/Components/W_StoreBrowser.Broswer Closed` _asw_store_browser (delegate `OnBrowserClosed`)))))

(event `OnBrowserClosed`
  ;[1 1 1] Launch payment console
  (`self.Check Pending Order` (stale `self.LaunchPaymentConsole` OrderId1) (stale `self.LaunchPaymentConsole` ResultHandler)))

(event `self.OnItemPurchaseInitiated`
  (params (Sku :type String) (ResultHandler :type "/Xsolla/Store/Handlers/BPI_PurchaseResultHandler Interface"))
  ;[1 1 1] Purchase item with real money
  (`/Xsolla/Common/BP_DemoUtils.ShowLoader` true)
  (`XsollaStoreSubsystem.FetchPaymentToken` :`self` (subsystem `XsollaStoreSubsystem`) :`AuthToken` (`/Xsolla/Login/Misc/BP_TokenUtils.GetToken`) :`ItemSKU` Sku :`SuccessCallback` (delegate `OnFetchItemPurchaseTokenSuccess`) :`ErrorCallback` (delegate `OnPurchaseItemError`)))

(event `OnFetchItemPurchaseTokenSuccess`
  (params (AccessToken :type String) (OrderId :type Integer))
  ;[1 1 1] Purchase item with real money
  (`/Xsolla/Common/BP_DemoUtils.ShowLoader` false)
  (`self.LaunchPaymentConsole` AccessToken OrderId (stale `self.OnItemPurchaseInitiated` ResultHandler)))

(event `Check Pending Order`
  (params (OrderId :type Integer) (ResultHandler :type "/Xsolla/Store/Handlers/BPI_PurchaseResultHandler Interface"))
  ;[1 1 1] check purchase status
  (bind _returnvalue (`XsollaStoreSubsystem.CreateOrderCheckObject` (subsystem `XsollaStoreSubsystem`) OrderId (delegate `OnCheckOrderStatusReceived`) (delegate `OnCheckOrderError`) (delegate `OnCheckOrderTimeoutError`) 300))
  (`KismetArrayLibrary.Array_Add` (`self.CachedOrderCheckObjects`) _returnvalue)
  (`XsollaOrderCheckObject.Connect` _returnvalue))

(event `OnPurchaseItemError`
  (params (StatusCode :type Integer) (ErrorCode :type Integer) (ErrorMessage :type String))
  ;[1 1 1] Purchase item with real money
  (`self.ShowError` StatusCode ErrorCode ErrorMessage)
  (`self.HandlePurchaseResult` (stale `self.OnItemPurchaseInitiated` ResultHandler) -1))

(event `OnCheckOrderStatusReceived`
  (params (OrderId :type Integer) (OrderStatus :type "EXsollaOrderStatus Enum" :default "Unknown"))
  ;[1 1 1] check purchase status
  (switch `EXsollaOrderStatus` OrderStatus
    (:`Paid`
      _)
    (:`Done`
      _))
  (`/Xsolla/Store/Handlers/BPI_PurchaseResultHandler.HandleResult` (stale `Check Pending Order` ResultHandler) (stale `Check Pending Order` OrderId) true)
  (`XsollaOrderCheckObject.Destroy` (stale `Check Pending Order` _returnvalue) :!label _label)
  (`KismetArrayLibrary.Array_RemoveItem` (`self.CachedOrderCheckObjects`) (stale `Check Pending Order` _returnvalue)))

(event `OnCheckOrderError`
  (params (ErrorMessage :type String))
  ;[1 1 1] check purchase status
  (`self.ShortPollingCheckOrder` (stale `Check Pending Order` OrderId) (stale `Check Pending Order` ResultHandler) :!label _label_2)
  (goto _label))

(event `OnCheckOrderTimeoutError`
  ;[1 1 1] check purchase status
  (goto _label_2))

(event `self.OnCartPurchaseInitiated`
  (params (CartId :type String) (ResultHandler :type "/Xsolla/Store/Handlers/BPI_PurchaseResultHandler Interface"))
  ;[1 1 1] Purchase cart with real money
  (`/Xsolla/Common/BP_DemoUtils.ShowLoader` true)
  (set `self.CachedCart` (`XsollaStoreSubsystem.GetCart` (subsystem `XsollaStoreSubsystem`)))
  (`XsollaStoreSubsystem.UpdateCart` (subsystem `XsollaStoreSubsystem`) (`/Xsolla/Login/Misc/BP_TokenUtils.GetToken`) CartId "" "" (delegate `OnUpdateCartBeforePurchaseSuccess`) (`|CreateDelegate` :!event `ShowError`)))

(event `OnUpdateCartBeforePurchaseSuccess`
  ;[1 1 1] Purchase cart with real money
  (if (`XsollaStoreLibrary.Equal_StoreCartStoreCart` (`self.CachedCart`) (`XsollaStoreSubsystem.GetCart` (subsystem `XsollaStoreSubsystem`)))
    (`XsollaStoreSubsystem.FetchCartPaymentToken` :`self` (subsystem `XsollaStoreSubsystem`) :`AuthToken` (`/Xsolla/Login/Misc/BP_TokenUtils.GetToken`) :`CartId` (stale `self.OnCartPurchaseInitiated` CartId) :`SuccessCallback` (delegate `OnFetchCartPurchaseTokenSuccess`) :`ErrorCallback` (`|CreateDelegate` :!event `ShowError`))
    (else
      (`/Xsolla/Common/BP_DemoUtils.ShowLoader` false)
      (`/Xsolla/Common/BP_DemoUtils.ShowMessagePopup` "The cart was updated, please check and retry" true))))

(event `ShortPollingCheckOrder`
  (params (OrderId :type Integer) (ResultHandler :type "/Xsolla/Store/Handlers/BPI_PurchaseResultHandler Interface"))
  ;[1 1 1] Purchase status polling
  (`XsollaStoreSubsystem.CheckOrder` :`self` (subsystem `XsollaStoreSubsystem`) :`AuthToken` (`/Xsolla/Login/Misc/BP_TokenUtils.GetToken`) :`OrderId` OrderId :`SuccessCallback` (delegate `On Check Order Success`)))

(event `OnRepeatCheck`
  ;[1 1 1] Purchase status polling
  (`self.ShortPollingCheckOrder` (stale `ShortPollingCheckOrder` OrderId) (stale `ShortPollingCheckOrder` ResultHandler)))

(event `On Check Order Success`
  (params (OrderId :type Integer) (OrderStatus :type "EXsollaOrderStatus Enum" :default "Unknown") (OrderContent :type "XsollaOrderContent Structure"))
  ;[1 1 1] Purchase status polling
  (switch `EXsollaOrderStatus` OrderStatus
    (:`New`
      (`KismetSystemLibrary.K2_SetTimerDelegate` (delegate `OnRepeatCheck`) 3.0))
    (:`Paid`
      (`/Xsolla/Store/Handlers/BPI_PurchaseResultHandler.HandleResult` (stale `ShortPollingCheckOrder` ResultHandler) (stale `ShortPollingCheckOrder` OrderId) true :!label _label_3))
    (:`Done`
      (goto _label_3))))

(event `OnFetchCartPurchaseTokenSuccess`
  (params (AccessToken :type String) (OrderId :type Integer))
  ;[1 1 1] Purchase cart with real money
  (`/Xsolla/Common/BP_DemoUtils.ShowLoader` false)
  (`self.LaunchPaymentConsole` AccessToken OrderId (stale `self.OnCartPurchaseInitiated` ResultHandler)))

(event `self.OnItemPurchaseVCInitiated`
  (params (Sku :type String) (CurrencySku :type String) (ResultHandler :type "/Xsolla/Store/Handlers/BPI_PurchaseResultHandler Interface"))
  ;[1 1 1] Purchase item with virtual currency
  (`/Xsolla/Common/BP_DemoUtils.ShowLoader` true)
  (`XsollaStoreSubsystem.BuyItemWithVirtualCurrency` (subsystem `XsollaStoreSubsystem`) (`/Xsolla/Login/Misc/BP_TokenUtils.GetToken`) Sku CurrencySku (delegate `OnPurchaseVCSuccess`) (delegate `OnVCPurchaseItemError`)))

(event `OnPurchaseVCSuccess`
  (params (OrderId :type Integer))
  ;[1 1 1] Purchase item with virtual currency
  (`/Xsolla/Common/BP_DemoUtils.ShowLoader` false)
  (`self.Check Pending Order` OrderId (stale `self.OnItemPurchaseVCInitiated` ResultHandler)))

(event `OnVCPurchaseItemError`
  (params (StatusCode :type Integer) (ErrorCode :type Integer) (ErrorMessage :type String))
  ;[1 1 1] Purchase item with virtual currency
  (`self.ShowError` StatusCode ErrorCode ErrorMessage)
  (`self.HandlePurchaseResult` (stale `self.OnItemPurchaseVCInitiated` ResultHandler) -1))

(fn `HandlePurchaseResult`
  (params (ResultHandler :type "/Xsolla/Store/Handlers/BPI_PurchaseResultHandler Interface") (OrderId :type Integer) (IsSuccess :type Boolean))
  (if (`KismetSystemLibrary.IsValid` (`KismetSystemLibrary.Conv_InterfaceToObject` ResultHandler))
    (`/Xsolla/Store/Handlers/BPI_PurchaseResultHandler.HandleResult` ResultHandler OrderId IsSuccess)))

(fn `Init`
  (params (InDemo :type "/Xsolla/Login/Interface/BPI_Demo Interface") (InDemoWidget :type "/Xsolla/Login/Interface/BPI_DemoWidget Interface"))
  (set `self.Demo` InDemo)
  (set `self.DemoWidget` InDemoWidget))

(fn `ShowError`
  (params (StatusCode :type Integer) (ErrorCode :type Integer) (ErrorMessage :type String))
  (`/Xsolla/Common/BP_DemoUtils.ShowLoader` false)
  (`/Xsolla/Common/BP_DemoUtils.ShowMessagePopup` (`KismetTextLibrary.Conv_StringToText` ErrorMessage) true))