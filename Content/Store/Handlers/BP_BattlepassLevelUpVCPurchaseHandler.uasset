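; Handles the results of Xsolla virtual currency purchases of battlepass level upgrades.
; Successful order IDs are collected until the request counter hits zero, then a self-recursing one-second delay loop polls each order and drops those marked Done.
; Once none remain, it consumes the inventory item, refreshes the currency balance and finishes the upgrade on the battlepass panel.
; Consume errors show a popup, while failed purchase results are ignored.
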(event `/Xsolla/Store/Handlers/BPI_PurchaseResultHandler.HandleResult`
  (params (OrderId :type Integer) (IsSuccess :type Boolean))
  (if IsSuccess
    (`KismetArrayLibrary.Array_Add` (`self.LevelUpgradePendingOrderIds`) OrderId)
    (bind _result (`/Engine/EditorBlueprintResources/StandardMacros.DecrementInt` (`self.LevelUpgradeCountRequests`))
      (:`  `
        (if (== _result 0)
          (`self.CheckPendingLevelUpgradeOrders`))))))

(event `CheckPendingLevelUpgradeOrders`
  (if (== (`KismetArrayLibrary.Array_Length` (`self.LevelUpgradePendingOrderIds`)) 0)
    (`self.OnBattlepassLevelUpgradeOrdersDone`)
    (else
      (`KismetSystemLibrary.Delay` 1.0)
      (for _array_element (`self.LevelUpgradePendingOrderIds`)
        (`XsollaStoreSubsystem.CheckOrder` :`self` (subsystem `XsollaStoreSubsystem`) :`AuthToken` (`/Xsolla/Login/Misc/BP_TokenUtils.GetToken`) :`OrderId` _array_element :`SuccessCallback` (delegate `OnBattlepassLevelUpgradeCheckOrderSuccess`)))
      (`self.CheckPendingLevelUpgradeOrders`))))

(event `OnBattlepassLevelUpgradeCheckOrderSuccess`
  (params (OrderId :type Integer) (OrderStatus :type "EXsollaOrderStatus Enum" :default "Unknown") (OrderContent :type "XsollaOrderContent Structure"))
  (if (`|EnumEquality` OrderStatus "Done")
    (`KismetArrayLibrary.Array_RemoveItem` (`self.LevelUpgradePendingOrderIds`) OrderId)))

(event `OnBattlepassLevelUpgradeOrdersDone`
  (`/Xsolla/Common/BP_DemoUtils.ShowLoader` false)
  (`XsollaInventorySubsystem.ConsumeInventoryItem` (subsystem `XsollaInventorySubsystem`) (`/Xsolla/Login/Misc/BP_TokenUtils.GetToken`) (`self.Sku`) (`self.Quantity`) "" (delegate `OnBattlepassUpgradeLevelItemConsumed`) (delegate `OnConsumeError`))
  (`/Xsolla/Inventory/Controllers/BPI_InventoryController.UpdateVirtualCurrencyBalance` (`self.InventoryController`) true))

(event `OnBattlepassUpgradeLevelItemConsumed`
  (`/Xsolla/Store/Interface/BPI_BattlepassPanel.FinishLevelUpgrade` (`self.BattlepassPanel`) true))

(event `OnConsumeError`
  (params (StatusCode :type Integer) (ErrorCode :type Integer) (ErrorMessage :type String))
  (`/Xsolla/Common/BP_DemoUtils.ShowLoader` false)
  (`/Xsolla/Common/BP_DemoUtils.ShowMessagePopup` (`KismetTextLibrary.Conv_StringToText` ErrorMessage) true))