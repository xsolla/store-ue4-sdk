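; BP_RefreshUserDataStoreHandler is an Xsolla store demo handler that refreshes the user's data when its HandleResult event fires.
; HandleResult updates the virtual currency balance through the InventoryController, requests the inventory and updates the cart from the Xsolla subsystems.
; When the cart update succeeds, it sums the cart item quantities and passes the total to the demo widget's cart counter.
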(event `/Xsolla/Common/Handlers/BPI_ResultHandler.HandleResult`
  (`/Xsolla/Inventory/Controllers/BPI_InventoryController.UpdateVirtualCurrencyBalance` (`self.InventoryController`) false)
  (`XsollaInventorySubsystem.GetInventory` :`self` (subsystem `XsollaInventorySubsystem`) :`AuthToken` (`/Xsolla/Login/Misc/BP_TokenUtils.GetToken`) :`Platform` "undefined")
  (`XsollaStoreSubsystem.UpdateCart` :`self` (subsystem `XsollaStoreSubsystem`) :`AuthToken` (`/Xsolla/Login/Misc/BP_TokenUtils.GetToken`) :`SuccessCallback` (delegate `OnInitialUpdateCartSuccess`)))

(event `OnInitialUpdateCartSuccess`
  (`self.RefreshCartCounter`))

(fn `RefreshCartCounter`
  (locals (CartCounter :type Integer))
  (bind (_returnvalue_cart_id _returnvalue_price _returnvalue_is_free _returnvalue_items) (break `StoreCart` (`XsollaStoreSubsystem.GetCart` (subsystem `XsollaStoreSubsystem`))))
  (for _array_element _returnvalue_items
    (set `local.CartCounter` (+ (`local.CartCounter`) (`.quantity` (break `StoreCartItem` _array_element)))))
  (`/Xsolla/Login/Interface/BPI_DemoWidget.RefreshCartCounter` (`self.DemoWidget`) (`local.CartCounter`)))