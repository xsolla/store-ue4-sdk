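; BP_BattlepassLevelUpRMPurchaseHandler handles the result of a battlepass level-up purchase, apparently made with real money.
; HandleResult consumes the purchased SKU and quantity through the Xsolla inventory subsystem, without branching on IsSuccess.
; On consumption, it passes IsSuccess to the battlepass panel's FinishLevelUpgrade.
; A consume error hides the loader and shows an error popup.
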(event `/Xsolla/Store/Handlers/BPI_PurchaseResultHandler.HandleResult`
  (params (OrderId :type Integer) (IsSuccess :type Boolean))
  (`XsollaInventorySubsystem.ConsumeInventoryItem` (subsystem `XsollaInventorySubsystem`) (`/Xsolla/Login/Misc/BP_TokenUtils.GetToken`) (`self.Sku`) (`self.Quantity`) "" (delegate `OnBattlepassUpgradeLevelItemConsumed`) (delegate `OnConsumeError`)))

(event `OnBattlepassUpgradeLevelItemConsumed`
  (`/Xsolla/Store/Interface/BPI_BattlepassPanel.FinishLevelUpgrade` (`self.BattlepassPanel`) (stale `/Xsolla/Store/Handlers/BPI_PurchaseResultHandler.HandleResult` IsSuccess)))

(event `OnConsumeError`
  (params (StatusCode :type Integer) (ErrorCode :type Integer) (ErrorMessage :type String))
  (`/Xsolla/Common/BP_DemoUtils.ShowLoader` false)
  (`/Xsolla/Common/BP_DemoUtils.ShowMessagePopup` (`KismetTextLibrary.Conv_StringToText` ErrorMessage) true))