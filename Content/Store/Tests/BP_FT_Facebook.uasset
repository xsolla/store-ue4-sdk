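; BP_FT_Facebook is a functional test that exercises the Facebook icon button in the UI.
; StartTest finds the button widget by name and triggers its click handler directly, waits on a fixed delay, then writes a hardcoded email address as text.
; It then finishes with success unconditionally, without verifying the outcome.
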(event `self.ReceiveStartTest`
  (`parent.ReceiveStartTest`)
  (bind _returnvalue (`TestHelper.FindUIElement` "W_IconButton_Facebook1" "/Xsolla/Common/Components/Primitives/W_IconButton.W_IconButton_C"))
  (`/Xsolla/Common/Components/Primitives/W_IconButton.OnIconButtonClicked` _returnvalue)
  (`KismetSystemLibrary.Delay` 10.0)
  (`TestHelper.WriteText` "peters2011.pm@gmail.com")
  (`TestHelper.FinishTest` null true "Success"))

(fn `UserConstructionScript`
  (`parent.UserConstructionScript`))