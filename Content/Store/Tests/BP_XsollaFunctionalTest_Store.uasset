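; Functional test base for the Xsolla store demo that opens the store items panel through the UI.
; On start it clicks the first demo user button, waits, clicks the Store button and waits again, finding widgets by name.
; It then checks that the main widget switcher shows the items panel, failing the test otherwise.
; On success it passes the panel to an empty ContinueTest event, apparently a hook for derived tests.
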(event `self.ReceivePrepareTest`
  (`parent.ReceivePrepareTest`))

(event `self.ReceiveStartTest`
  (`parent.ReceiveStartTest`)
  (bind _returnvalue (`TestHelper.FindUIElementByName` "W_ButtonWrapper_DemoUser1" "/Xsolla/Common/Components/Wrappers/W_ButtonWrapper.W_ButtonWrapper_C"))
  (`/Xsolla/Common/Components/Wrappers/W_ButtonWrapper.OnClicked` _returnvalue)
  (`KismetSystemLibrary.Delay` 7.0)
  (bind _returnvalue_2 (`TestHelper.FindUIElementByName` "W_ButtonWrapper_Store" "/Xsolla/Common/Components/Wrappers/W_ButtonWrapper.W_ButtonWrapper_C"))
  (`/Xsolla/Common/Components/Wrappers/W_ButtonWrapper.OnClicked` _returnvalue_2)
  (`KismetSystemLibrary.Delay` 5.0)
  (bind _returnvalue_3 (`TestHelper.FindUIElementByName` "WidgetSwitcher_Main" "/Script/UMG.WidgetSwitcher"))
  (bind _returnvalue_4 (`WidgetSwitcher.GetActiveWidget` _returnvalue_3))
  (if (`KismetStringLibrary.EqualEqual_StrStr` (`KismetSystemLibrary.GetObjectName` _returnvalue_4) "W_StorePanel_Items")
    (bind _asw_store_panel (cast `/Xsolla/Store/Panels/W_StorePanel` _returnvalue_4)
      (:`then`
        (`self.ContinueTest` _asw_store_panel))
      (:`CastFailed`
        (`self.FinishTest` "Failed" "W_StorePanel_Items not opened" :!label _label)))
    (else
      (goto _label))))

(event `ContinueTest`
  (params (StoreItemsWidget :type "/Xsolla/Store/Panels/W_StorePanel Object Reference")))

(fn `UserConstructionScript`
  (`parent.UserConstructionScript`))