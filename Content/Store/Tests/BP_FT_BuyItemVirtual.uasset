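; Functional test that buys a store item with virtual currency through the store UI.
; ContinueTest finds the configured SKU in the store tile list, reads its currency SKU and starts the purchase.
; It clicks the confirm popup's button after a short delay, then waits and passes only if the message popup's title reads "Success".
; A GetQueryString helper builds a JavaScript field-setting string but is not called here.
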(event `self.ReceiveStartTest`
  (`parent.ReceiveStartTest`))

(event `self.ContinueTest`
  (params (StoreItemsWidget :type "/Xsolla/Store/Panels/W_StorePanel Object Reference"))
  (bind _sku (`/Xsolla/Store/Tests/BPFL_StoreTests.GetBuyForVirtualSku`))
  (for _array_element (`ListView.GetListItems` (`/Xsolla/Store/Panels/W_StorePanel.TileView_Store` StoreItemsWidget))
    (bind _asbpi_store_item_data (cast `/Xsolla/Store/Interface/BPI_StoreItemData` _array_element))
    (bind _sku_2 (`/Xsolla/Store/Interface/BPI_StoreItemData.GetSku` _asbpi_store_item_data))
    (if (`KismetStringLibrary.EqualEqual_StrStr` _sku_2 _sku)
      (bind _price (`/Xsolla/Store/Interface/BPI_StoreItemData.GetPriceVC` _asbpi_store_item_data))
      (bind _sku_3 (`/Xsolla/Store/Interface/BPI_VCPrice.GetSku` _price))
      (set `self.CurrencySku` _sku_3)
      (set `self.bSkuWasFound` true)))
  (if (`self.bSkuWasFound`)
    (`/Xsolla/Store/Panels/W_StorePanel.PurchaseItemVC` StoreItemsWidget _sku (`self.CurrencySku`))
    (`KismetSystemLibrary.Delay` 0.2)
    (bind _returnvalue (`TestHelper.FindWidgetByClass` "/Xsolla/Common/Popup/W_ConfirmPopup.W_ConfirmPopup_C"))
    (`/Engine/EditorBlueprintResources/StandardMacros.IsValid` _returnvalue
      (:`Is Valid`
        (bind _returnvalue_2 (`TestHelper.FindUIElementInWidgetByName` _returnvalue "W_ButtonWrapper_Confirm" "/Xsolla/Common/Components/Wrappers/W_ButtonWrapper.W_ButtonWrapper_C"))
        (`/Xsolla/Common/Components/Wrappers/W_ButtonWrapper.OnClicked` _returnvalue_2)
        (`KismetSystemLibrary.Delay` 3.0)
        (bind _returnvalue_3 (`TestHelper.FindWidgetByClass` "/Xsolla/Common/Popup/W_MessagePopup.W_MessagePopup_C"))
        (`/Engine/EditorBlueprintResources/StandardMacros.IsValid` _returnvalue_3
          (:`Is Valid`
            (bind _returnvalue_4 (`TestHelper.FindUIElementInWidgetByName` _returnvalue_3 "W_TextWrapper_Title" "/Xsolla/Common/Components/Wrappers/W_TextWrapper.W_TextWrapper_C"))
            (bind _text (`/Xsolla/Common/Components/Wrappers/W_TextWrapper.GetText` _returnvalue_4))
            (`TestHelper.FinishTest` null (`KismetStringLibrary.EqualEqual_StrStr` (`KismetTextLibrary.Conv_TextToString` _text) "Success") "Success buy virtual item!" "Item was not purchased"))
          (:`Is Not Valid`
            (`self.FinishTest` "Failed" "Popup did not appear"))))
      (:`Is Not Valid`
        (`self.FinishTest` "Failed" "Confirm popup did not appear")))
    (else
      (`self.FinishTest` "Failed" (`KismetStringLibrary.Concat_StrStr` "Can't find item with sku " _sku)))))

(fn `GetQueryString`
  (params (type :type String) (id :type String) (value :type String))
  (returns (result :type String))
  (return (`KismetTextLibrary.Conv_TextToString` (`|FormatText` "document.querySelector(\"{type}[id='{Id}']\").value = \"{Value}\"" type id value))))

(fn `UserConstructionScript`
  (`parent.UserConstructionScript`))