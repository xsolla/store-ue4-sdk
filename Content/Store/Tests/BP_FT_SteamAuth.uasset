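; Functional test that checks store demo login with Steam authorization enabled in the login settings.
; SetupProjectSettings turns on the Steam authorization flag after calling the parent setup.
; StartTest fills the username and password widgets with test credentials and triggers the login button through UI lookup helpers.
; After a fixed delay, it passes if a W_StoreDemo widget exists and fails otherwise.
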(event `self.ReceiveStartTest`
  (`parent.ReceiveStartTest`)
  (`TestHelper.SetInputFieldText` "W_Input_Username" (`KismetTextLibrary.Conv_StringToText` "xsolla") true)
  (`TestHelper.SetInputFieldText` "W_Input_Password" (`KismetTextLibrary.Conv_StringToText` "xsolla") true)
  (bind _returnvalue (`TestHelper.FindUIElement` "W_Button_Login" "/Xsolla/Common/Components/Primitives/W_Button.W_Button_C"))
  (`/Xsolla/Common/Components/Primitives/W_Button.OnClicked` _returnvalue)
  (`KismetSystemLibrary.Delay` 3.0)
  (bind _returnvalue_2 (`TestHelper.FindWidgetByClass` "/Xsolla/Store/W_StoreDemo.W_StoreDemo_C"))
  (`/Engine/EditorBlueprintResources/StandardMacros.IsValid` _returnvalue_2
    (:`Is Valid`
      (`self.FinishTest` "Succeeded" "Success store login"))
    (:`Is Not Valid`
      (`self.FinishTest` "Failed" "StoreWidget not found"))))

(fn `SetupProjectSettings`
  (`parent.SetupProjectSettings`)
  (set `XsollaLoginSettings.bUseSteamAuthorization` true (`XsollaLoginLibrary.GetLoginSettings`)))

(fn `UserConstructionScript`
  (`parent.UserConstructionScript`))