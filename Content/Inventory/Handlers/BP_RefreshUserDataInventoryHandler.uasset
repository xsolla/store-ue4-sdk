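; BP_RefreshUserDataInventoryHandler is an inventory handler in the Xsolla demo that reacts to the result of a user data refresh.
; It updates the virtual currency balance through the inventory controller, then refreshes the inventory widget's account linking status unless custom auth via access token is on.
; Linking counts as required when a store demo exists, cross-platform linking is enabled, the platform isn't PlayStation Network and the account isn't master.
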(event `/Xsolla/Common/Handlers/BPI_ResultHandler.HandleResult`
  (`/Xsolla/Inventory/Controllers/BPI_InventoryController.UpdateVirtualCurrencyBalance` (`self.InventoryController`) false)
  (if (not (`XsollaLoginSettings.bCustomAuthViaAccessToken` (`XsollaLoginLibrary.GetLoginSettings`)))
    (`/Xsolla/Inventory/W_InventoryWidget.RefreshAccountLinkingStatus` (`self.InventoryWidget`) (not (`self.IsAccountLinkingRequired`)))))

(fn `IsAccountLinkingRequired`
  (returns (IsLinkingRequired :type Boolean))
  (bind _returnvalue (`XsollaLoginLibrary.GetLoginSettings`))
  (bind _asxsolla_demo_game_mode_base (cast `/Xsolla/Common/XsollaDemoGameModeBase` (`GameplayStatics.GetGameMode`)))
  (return (and (`KismetSystemLibrary.IsValidClass` (`XsollaDemoGameModeBase.GetStoreDemo` _asxsolla_demo_game_mode_base)) (`XsollaLoginSettings.UseCrossPlatformAccountLinking` _returnvalue) (`|EnumInequality` (`XsollaLoginSettings.Platform` _returnvalue) "playstation_network") (not (`/Xsolla/Login/Misc/BP_TokenUtils.IsMasterAccount`)))))