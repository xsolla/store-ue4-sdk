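; Base functional test for the Xsolla inventory UI that navigates from demo login to the inventory panel.
; On start, it finds the DemoUser1 and Inventory buttons by name and fires their click handlers, with fixed delays after each.
; It then passes the main switcher's active W_InventoryPanel to an empty ContinueTest event, or fails the test if that panel is not open.
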(event `self.ReceivePrepareTest`
  (`parent.ReceivePrepareTest`))

(event `self.ReceiveStartTest`
  (`parent.ReceiveStartTest`)
  (bind _returnvalue (`TestHelper.FindUIElementByName` "W_ButtonWrapper_DemoUser1" "/Xsolla/Common/Components/Wrappers/W_ButtonWrapper.W_ButtonWrapper_C"))
  (`/Xsolla/Common/Components/Wrappers/W_ButtonWrapper.OnClicked` _returnvalue)
  (`KismetSystemLibrary.Delay` 3.0)
  (bind _returnvalue_2 (`TestHelper.FindUIElementByName` "W_ButtonWrapper_Inventory" "/Xsolla/Common/Components/Wrappers/W_ButtonWrapper.W_ButtonWrapper_C"))
  (`/Xsolla/Common/Components/Wrappers/W_ButtonWrapper.OnClicked` _returnvalue_2)
  (`KismetSystemLibrary.Delay` 3.0)
  (bind _returnvalue_3 (`TestHelper.FindUIElementByName` "WidgetSwitcher_Main" "/Script/UMG.WidgetSwitcher"))
  (bind _returnvalue_4 (`WidgetSwitcher.GetActiveWidget` _returnvalue_3))
  (if (`KismetStringLibrary.EqualEqual_StrStr` (`KismetSystemLibrary.GetObjectName` _returnvalue_4) "W_InventoryPanel")
    (bind _asw_inventory_panel (cast `/Xsolla/Inventory/Panels/W_InventoryPanel` _returnvalue_4)
      (:`then`
        (`self.ContinueTest` _asw_inventory_panel))
      (:`CastFailed`
        (`self.FinishTest` "Failed" "W_InventoryPanel not opened" :!label _label)))
    (else
      (goto _label))))

(event `ContinueTest`
  (params (InventoryWidget :type "/Xsolla/Inventory/Panels/W_InventoryPanel Object Reference")))

(fn `UserConstructionScript`
  (`parent.UserConstructionScript`))