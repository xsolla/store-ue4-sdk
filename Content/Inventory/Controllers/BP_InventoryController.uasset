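; Inventory controller for the Xsolla demo, linking XsollaInventorySubsystem to the demo's inventory and currency UI.
; Panel refresh chains inventory and subscription requests, then builds non-currency item objects with expiry times and loads their icons.
; Coupon redemption and item consumption run through popups and success callbacks, then refresh the panel; redemption also updates virtual currency balances.
; IsItemInInventory is a stub that always returns false.
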(event `self.RefreshInventoryPanel`
  (params (ActivateWhenReady :type Boolean) (Panel :type "/Xsolla/Inventory/Interface/BPI_InventoryPanel Interface"))
  ;[1 1 1] Refresh inventory panel
  (`/Xsolla/Common/BP_DemoUtils.ShowLoader` true)
  (`XsollaInventorySubsystem.UpdateInventory` (subsystem `XsollaInventorySubsystem`) (`/Xsolla/Login/Misc/BP_TokenUtils.GetToken`) "undefined" (delegate `OnUpdateInventorySuccess`) (`|CreateDelegate` :!event `ShowError`) 50 0))

(event `OnUpdateInventorySuccess`
  (params (InventoryData :type "InventoryItemsData Structure (by ref)"))
  ;[1 1 1] Refresh inventory panel
  (set `self.Inventory Data` InventoryData)
  (`XsollaInventorySubsystem.UpdateSubscriptions` (subsystem `XsollaInventorySubsystem`) (`/Xsolla/Login/Misc/BP_TokenUtils.GetToken`) "undefined" (delegate `OnUpdateSubscriptionsSuccess`) (`|CreateDelegate` :!event `ShowError`)))

(event `OnUpdateSubscriptionsSuccess`
  (params (SubscriptionData :type "SubscriptionData Structure (by ref)"))
  ;[1 1 1] Refresh inventory panel
  (set `self.Subscription Data` SubscriptionData)
  (`/Xsolla/Common/BP_DemoUtils.ShowLoader` false)
  (bind _inventorydata (`self.CreateInventoryData` (stale `self.RefreshInventoryPanel` Panel)))
  (`/Xsolla/Inventory/Interface/BPI_InventoryPanel.RefreshInventoryItemsList` (stale `self.RefreshInventoryPanel` Panel) _inventorydata)
  (if (stale `self.RefreshInventoryPanel` ActivateWhenReady)
    (`/Xsolla/Login/Interface/BPI_DemoWidget.ActivateInventoryPanel` (`self.DemoWidget`))))

(event `self.OnRedeemCouponInitiated`
  (params (Panel :type "/Xsolla/Inventory/Interface/BPI_InventoryPanel Interface"))
  ;[1 1 1] Redeem coupon
  (bind _returnvalue (`|CreateWidget` "/Xsolla/Inventory/Popup/W_RedeemCouponPopup.W_RedeemCouponPopup_C" (`GameplayStatics.GetPlayerController` 0)))
  (`UserWidget.AddToViewport` _returnvalue 10000)
  (add `/Xsolla/Inventory/Popup/W_RedeemCouponPopup.OnPopupResult` _returnvalue (delegate `OnRedeemPopupResult`)))

(event `OnRedeemPopupResult`
  (params (IsConfirmed :type Boolean) (Code :type String))
  ;[1 1 1] Redeem coupon
  (if IsConfirmed
    (`XsollaInventorySubsystem.RedeemCoupon` (subsystem `XsollaInventorySubsystem`) (`/Xsolla/Login/Misc/BP_TokenUtils.GetToken`) Code (delegate `OnCouponRedeemSuccess`) (delegate `OnCouponRedeemError`))))

(event `OnCouponRedeemSuccess`
  (params (RewardData :type "InventoryRedeemedCouponData Structure"))
  ;[1 1 1] Redeem coupon
  (`Widget.RemoveFromParent` (stale `self.OnRedeemCouponInitiated` _returnvalue))
  (bind _rewardsdata (`self.CreateCouponRewardData` RewardData))
  (bind _returnvalue (`|CreateWidget` "/Xsolla/Inventory/Popup/W_RedeemedCouponRewardsPopup.W_RedeemedCouponRewardsPopup_C" (`GameplayStatics.GetPlayerController` 0) _rewardsdata))
  (`UserWidget.AddToViewport` _returnvalue 10000)
  (`KismetSystemLibrary.Delay` 1.0)
  (`self.UpdateVirtualCurrencyBalance` false)
  (`self.RefreshInventoryPanel` false (stale `self.OnRedeemCouponInitiated` Panel)))

(event `OnCouponRedeemError`
  (params (StatusCode :type Integer) (ErrorCode :type Integer) (ErrorMessage :type String))
  ;[1 1 1] Redeem coupon
  (`/Xsolla/Inventory/Popup/W_RedeemCouponPopup.SetErrorState` (stale `self.OnRedeemCouponInitiated` _returnvalue) true))

(event `self.OnItemConsumptionInitiated`
  (params (Sku :type String) (InstanceId :type String) (Quantity :type Integer) (Panel :type "/Xsolla/Inventory/Interface/BPI_InventoryPanel Interface"))
  ;[1 1 1] Consume inventory item
  (bind _returnvalue (`|CreateWidget` "/Xsolla/Common/Popup/W_ConfirmPopup.W_ConfirmPopup_C" (`GameplayStatics.GetPlayerController` 0) (`|FormatText` "Are you sure you want to consume  {ItemName}?" (`self.GetItemName` Sku)) "CONFIRM"))
  (`UserWidget.AddToViewport` _returnvalue 10000)
  (add `/Xsolla/Common/Popup/W_ConfirmPopup.OnPopupResult` _returnvalue (delegate `OnConsumptionConfirmResult`)))

(event `OnConsumptionConfirmResult`
  (params (IsConfirmed :type Boolean))
  ;[1 1 1] Consume inventory item
  (if IsConfirmed
    (`/Xsolla/Common/BP_DemoUtils.ShowLoader` true)
    (`XsollaInventorySubsystem.ConsumeInventoryItem` (subsystem `XsollaInventorySubsystem`) (`/Xsolla/Login/Misc/BP_TokenUtils.GetToken`) (stale `self.OnItemConsumptionInitiated` Sku) (stale `self.OnItemConsumptionInitiated` Quantity) (stale `self.OnItemConsumptionInitiated` InstanceId) "undefined" (delegate `OnConsumeSuccess`) (`|CreateDelegate` :!event `ShowError`))))

(event `OnConsumeSuccess`
  ;[1 1 1] Consume inventory item
  (`/Xsolla/Common/BP_DemoUtils.ShowLoader` false)
  (`/Xsolla/Common/BP_DemoUtils.ShowMessagePopup` (`|FormatText` "You have consumed '{ItemName}' x {Quantity}!" (`self.GetItemName` (stale `self.OnItemConsumptionInitiated` Sku)) (stale `self.OnItemConsumptionInitiated` Quantity)) false self)
  (`self.RefreshInventoryPanel` false (stale `self.OnItemConsumptionInitiated` Panel)))

(event `self.UpdateVirtualCurrencyBalance`
  (params (bShowLoader :type Boolean))
  ;[1 1 1] update virtual currency balance
  (if bShowLoader
    (`/Xsolla/Common/BP_DemoUtils.ShowLoader` true))
  (`XsollaInventorySubsystem.UpdateVirtualCurrencyBalance` (subsystem `XsollaInventorySubsystem`) (`/Xsolla/Login/Misc/BP_TokenUtils.GetToken`) "undefined" (delegate `OnUpdateVirtualCurrencyBalanceSuccess`) (delegate `OnUpdateVirtuaCurrencyBalanceError`)))

(event `OnUpdateVirtualCurrencyBalanceSuccess`
  (params (CurrencyBalanceData :type "VirtualCurrencyBalanceData Structure (by ref)"))
  ;[1 1 1] update virtual currency balance
  (set `self.Currency Balance Data` CurrencyBalanceData)
  (if (stale `self.UpdateVirtualCurrencyBalance` bShowLoader)
    (`/Xsolla/Common/BP_DemoUtils.ShowLoader` false))
  (bind _balancedata (`self.CreateVCBalanceData`))
  (`/Xsolla/Login/Interface/BPI_DemoWidget.RefreshVirtualCurrencyBalance` (`self.DemoWidget`) _balancedata))

(event `OnUpdateVirtuaCurrencyBalanceError`
  (params (StatusCode :type Integer) (ErrorCode :type Integer) (ErrorMessage :type String))
  ;[1 1 1] update virtual currency balance
  (if (stale `self.UpdateVirtualCurrencyBalance` bShowLoader)
    (`/Xsolla/Common/BP_DemoUtils.ShowLoader` false)))

(fn `CreateCouponRewardData`
  (params (StoreRedeemedCouponData :type "InventoryRedeemedCouponData Structure (by ref)"))
  (returns (RewardsData :type "Array of /Xsolla/Inventory/Interface/BPI_CouponRewardItemData Interface"))
  (locals (RewardItems :type "Array of /Xsolla/Inventory/Interface/BPI_CouponRewardItemData Interface") (IconPresenters :type "Array of /Xsolla/Common/Interface/BPI_IconPresenter Interface"))
  (for _array_element (`.items` (break `InventoryRedeemedCouponData` StoreRedeemedCouponData))
    (bind _returnvalue (`|GenericCreateObject` "/Xsolla/Inventory/Data/BP_CouponRewardItemData.BP_CouponRewardItemData_C" (`GameplayStatics.GetPlayerController` self) _array_element))
    (`KismetArrayLibrary.Array_Add` (`local.RewardItems`) _returnvalue)
    (`KismetArrayLibrary.Array_Add` (`local.IconPresenters`) _returnvalue))
  (bind _iconsloader (`/Xsolla/Login/Interface/BPI_Demo.GetIconsLoader` (`self.Demo`)))
  (`/Xsolla/Login/Interface/BPI_IconsLoader.LoadIcons` _iconsloader (`local.IconPresenters`))
  (return (`local.RewardItems`)))

(fn `CreateInventoryData`
  (params (Inventory :type "/Xsolla/Inventory/Interface/BPI_InventoryPanel Interface"))
  (returns (InventoryData :type "Array of /Xsolla/Inventory/Interface/BPI_InventoryItemData Interface"))
  (locals (InventoryItemData :type "Array of /Xsolla/Inventory/Interface/BPI_InventoryItemData Interface") (IconPresenters :type "Array of /Xsolla/Common/Interface/BPI_IconPresenter Interface"))
  (for _array_element (`.Items` (break `InventoryItemsData` (`self.Inventory Data`)))
    (bind (_sku _name _type) (break `InventoryItem` _array_element))
    (if (`KismetStringLibrary.NotEqual_StrStr` "virtual_currency" _type)
      (bind _returnvalue (`|GenericCreateObject` "/Xsolla/Inventory/Data/BP_InventoryItemData.BP_InventoryItemData_C" (`GameplayStatics.GetPlayerController` self) (`self.GetSubscriptionExpirationTime` _sku) Inventory _array_element))
      (`KismetArrayLibrary.Array_Add` (`local.InventoryItemData`) _returnvalue)
      (`KismetArrayLibrary.Array_Add` (`local.IconPresenters`) _returnvalue)))
  (bind _iconsloader (`/Xsolla/Login/Interface/BPI_Demo.GetIconsLoader` (`self.Demo`)))
  (`/Xsolla/Login/Interface/BPI_IconsLoader.LoadIcons` _iconsloader (`local.IconPresenters`))
  (return (`local.InventoryItemData`)))

(fn `CreateVCBalanceData`
  (returns (BalanceData :type "Array of /Xsolla/Inventory/Interface/BPI_VCBalanceItemData Interface"))
  (locals (VCBalanceData :type "Array of /Xsolla/Inventory/Interface/BPI_VCBalanceItemData Interface") (IconPresenters :type "Array of /Xsolla/Common/Interface/BPI_IconPresenter Interface"))
  (bind _currency_balance_data_items (break `VirtualCurrencyBalanceData` (`self.Currency Balance Data`)))
  (for _array_element _currency_balance_data_items
    (bind _returnvalue (`|GenericCreateObject` "/Xsolla/Inventory/Data/BP_VCBalanceItemData.BP_VCBalanceItemData_C" (`GameplayStatics.GetPlayerController` 0) _array_element))
    (`KismetArrayLibrary.Array_Add` (`local.VCBalanceData`) _returnvalue)
    (`KismetArrayLibrary.Array_Add` (`local.IconPresenters`) _returnvalue))
  (bind _iconsloader (`/Xsolla/Login/Interface/BPI_Demo.GetIconsLoader` (`self.Demo`)))
  (`/Xsolla/Login/Interface/BPI_IconsLoader.LoadIcons` _iconsloader (`local.IconPresenters`))
  (return (`local.VCBalanceData`)))

(fn `GetItemName`
  (params (ItemSKU :type String))
  (returns (Name :type String))
  (bind _inventory_data_items (break `InventoryItemsData` (`self.Inventory Data`)))
  (for _array_element _inventory_data_items
    (bind (_sku _name) (break `InventoryItem` _array_element))
    (if (`KismetStringLibrary.EqualEqual_StrStr` ItemSKU _sku)
      (return _name)))
  (return ""))

(fn `GetSubscriptionExpirationTime`
  (params (Sku :type String))
  (returns (ExpiresAt :type Integer64))
  (bind _subscription_data_items (break `SubscriptionData` (`self.Subscription Data`)))
  (for _array_element _subscription_data_items
    (bind (_sku _name _type _virtual_item_type _description _image_url _expired_at) (break `SubscriptionItem` _array_element))
    (if (`KismetStringLibrary.EqualEqual_StrStr` Sku _sku)
      (return _expired_at)))
  (return 0))

(fn `Init`
  (params (InDemo :type "/Xsolla/Login/Interface/BPI_Demo Interface") (InDemoWidget :type "/Xsolla/Login/Interface/BPI_DemoWidget Interface"))
  (set `self.Demo` InDemo)
  (set `self.DemoWidget` InDemoWidget)
  (`XsollaInventorySubsystem.Initialize` (subsystem `XsollaInventorySubsystem`) (select `bool` (`/Xsolla/Common/BP_DemoUtils.Does Dev Menu Save Game Exist`) :`false` (`XsollaProjectSettings.ProjectID` (`XsollaSettingsLibrary.GetProjectSettings`)) :`true` (`.ProjectID_10_F159CBC8422282C5B7D45F8672FE9D4F` (break `/Xsolla/Common/Misc/XsollaDevMenuData` (`/Xsolla/Common/BP_DemoUtils.LoadDevMenuData`))))))

(fn `IsItemInInventory`
  (params (ItemSKU :type String))
  (returns (IsInInventory :type Boolean))
  (return false))

(fn `ShowError`
  (params (StatusCode :type Integer) (ErrorCode :type Integer) (ErrorMessage :type String))
  (`/Xsolla/Common/BP_DemoUtils.ShowLoader` false)
  (`/Xsolla/Common/BP_DemoUtils.ShowMessagePopup` (`KismetTextLibrary.Conv_StringToText` ErrorMessage) true))