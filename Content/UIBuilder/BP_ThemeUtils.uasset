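; BP_ThemeUtils is a UI helper library that reads colors, fonts and brushes from a theme and applies them to widgets.
; Color and font getters look up entries by name or by type, returning a caller-supplied default when the theme is invalid.
; Button and input field updaters, also in name and type variants, rebuild widget styles from theme brushes while preserving properties like padding.
; Input fields also take themed fonts at a given size and text color, with Roboto and translucent white as fallbacks.
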(fn `GetColor`
  (params (Theme :type "XsollaUIBuilderTheme Class Reference") (ColorType :type "EColorType Enum" :default "ColorType_Default") (DefaultColor :type "SlateColor Structure"))
  (returns (Color :type "SlateColor Structure"))
  (bind _returnvalue (`XsollaUIBuilderLibrary.GetTheme` Theme))
  (if (`KismetSystemLibrary.IsValid` _returnvalue)
    (return (make `SlateColor` (`KismetMathLibrary.Conv_ColorToLinearColor` (`XsollaUIBuilderTheme.GetColorByType` _returnvalue ColorType))))
    (else
      (return DefaultColor))))

(fn `GetFont`
  (params (Theme :type "XsollaUIBuilderTheme Class Reference") (FontType :type "EFontType Enum" :default "FontType_Default") (DefaultFont :type "SlateFontInfo Structure"))
  (returns (ReturnValue :type "SlateFontInfo Structure (by ref)"))
  (bind _returnvalue (`XsollaUIBuilderLibrary.GetTheme` Theme))
  (if (`KismetSystemLibrary.IsValid` _returnvalue)
    (return (`XsollaUIBuilderTheme.GetFontByType` _returnvalue FontType))
    (else
      (return DefaultFont))))

(fn `GetThemeColor`
  (params (Theme :type "XsollaUIBuilderTheme Class Reference") (ColorName :type String) (DefaultColor :type "SlateColor Structure"))
  (returns (Color :type "SlateColor Structure"))
  (bind _returnvalue (`XsollaUIBuilderLibrary.GetTheme` Theme))
  (if (`KismetSystemLibrary.IsValid` _returnvalue)
    (return (make `SlateColor` (`KismetMathLibrary.Conv_ColorToLinearColor` (`XsollaUIBuilderTheme.GetColor` _returnvalue ColorName))))
    (else
      (return DefaultColor))))

(fn `GetThemeFont`
  (params (Theme :type "XsollaUIBuilderTheme Class Reference") (FontName :type String) (DefaultFont :type "SlateFontInfo Structure"))
  (returns (ReturnValue :type "SlateFontInfo Structure (by ref)"))
  (bind _returnvalue (`XsollaUIBuilderLibrary.GetTheme` Theme))
  (if (`KismetSystemLibrary.IsValid` _returnvalue)
    (return (`XsollaUIBuilderTheme.GetFont` _returnvalue FontName))
    (else
      (return DefaultFont))))

(fn `UpdateButtonStyle`
  (params (Theme :type "XsollaUIBuilderTheme Class Reference") (NormalStateBrush :type String) (HoverStateBrush :type String) (PressedStateBrush :type String) (DisabledStateBrush :type String) (Button :type "Button Object Reference"))
  (bind _returnvalue (`XsollaUIBuilderLibrary.GetTheme` Theme))
  (bind (_normal _hovered _pressed _disabled _normalpadding _pressedpadding _pressedslatesound _hoveredslatesound) (break `ButtonStyle` (`Button.WidgetStyle` Button)))
  (`/Engine/EditorBlueprintResources/StandardMacros.IsValid` _returnvalue
    (:`Is Valid`
      (`Button.SetStyle` Button (make `ButtonStyle` (`XsollaUIBuilderTheme.GetBrush` _returnvalue NormalStateBrush) (`XsollaUIBuilderTheme.GetBrush` _returnvalue HoverStateBrush) (`XsollaUIBuilderTheme.GetBrush` _returnvalue PressedStateBrush) (`XsollaUIBuilderTheme.GetBrush` _returnvalue DisabledStateBrush) _normalpadding _pressedpadding _pressedslatesound _hoveredslatesound)))))

(fn `UpdateButtonThemeStyle`
  (params (Theme :type "XsollaUIBuilderTheme Class Reference") (NormalStateType :type "EBrushThemeType Enum" :default "BrushType_Default") (HoverStateType :type "EBrushThemeType Enum" :default "BrushType_Default") (PressedStateType :type "EBrushThemeType Enum" :default "BrushType_Default") (DisabledStateType :type "EBrushThemeType Enum" :default "BrushType_Default") (Button :type "Button Object Reference"))
  (bind _returnvalue (`XsollaUIBuilderLibrary.GetTheme` Theme))
  (bind (_normal _hovered _pressed _disabled _normalpadding _pressedpadding _pressedslatesound _hoveredslatesound) (break `ButtonStyle` (`Button.WidgetStyle` Button)))
  (`/Engine/EditorBlueprintResources/StandardMacros.IsValid` _returnvalue
    (:`Is Valid`
      (`Button.SetStyle` Button (make `ButtonStyle` (`XsollaUIBuilderTheme.GetBrushByType` _returnvalue NormalStateType) (`XsollaUIBuilderTheme.GetBrushByType` _returnvalue HoverStateType) (`XsollaUIBuilderTheme.GetBrushByType` _returnvalue PressedStateType) (`XsollaUIBuilderTheme.GetBrushByType` _returnvalue DisabledStateType) _normalpadding _pressedpadding _pressedslatesound _hoveredslatesound)))))

(fn `UpdateInputFieldStyle`
  (params (Theme :type "XsollaUIBuilderTheme Class Reference") (NormalStateBrush :type String) (HoverStateBrush :type String) (ActiveStateBrush :type String) (DisabledStateBrush :type String) (FontName :type String) (FontSize :type Integer) (TextColor :type String) (InputField :type "EditableTextBox Object Reference"))
  (bind _returnvalue (`XsollaUIBuilderLibrary.GetTheme` Theme))
  (bind (_backgroundimagenormal _backgroundimagehovered _backgroundimagefocused _backgroundimagereadonly _padding _font _foregroundcolor _backgroundcolor _readonlyforegroundcolor _hscrollbarpadding _vscrollbarpadding _scrollbarstyle) (break `EditableTextBoxStyle` (`EditableTextBox.WidgetStyle` InputField)))
  (bind (_fontobject _fontmaterial _outlinesettings _typefacefontname _size _letterspacing) (break `SlateFontInfo` (`self.GetThemeFont` Theme FontName (make `SlateFontInfo` "/Xsolla/Common/Assets/Font/Font_Roboto-Regular.Font_Roboto-Regular" null (struct :`OutlineColor` (struct :`A` 1.0)) "None" 14))))
  (`/Engine/EditorBlueprintResources/StandardMacros.IsValid` _returnvalue
    (:`Is Valid`
      (set `EditableTextBox.WidgetStyle` (make `EditableTextBoxStyle` (`XsollaUIBuilderTheme.GetBrush` _returnvalue NormalStateBrush) (`XsollaUIBuilderTheme.GetBrush` _returnvalue HoverStateBrush) (`XsollaUIBuilderTheme.GetBrush` _returnvalue ActiveStateBrush) (`XsollaUIBuilderTheme.GetBrush` _returnvalue DisabledStateBrush) _padding (make `SlateFontInfo` _fontobject _fontmaterial _outlinesettings _typefacefontname FontSize _letterspacing) (`self.GetThemeColor` Theme TextColor (make `SlateColor` (struct :`R` 1.0 :`G` 1.0 :`B` 1.0 :`A` 0.7))) _backgroundcolor _readonlyforegroundcolor _hscrollbarpadding _vscrollbarpadding _scrollbarstyle) InputField))))

(fn `UpdateInputFieldThemeStyle`
  (params (Theme :type "XsollaUIBuilderTheme Class Reference") (NormalStateBrush :type "EBrushThemeType Enum" :default "BrushType_Default") (HoverStateBrush :type "EBrushThemeType Enum" :default "BrushType_Default") (ActiveStateBrush :type "EBrushThemeType Enum" :default "BrushType_Default") (DisabledStateBrush :type "EBrushThemeType Enum" :default "BrushType_Default") (FontType :type "EFontType Enum" :default "FontType_Default") (FontSize :type Integer) (TextColor :type "EColorType Enum" :default "ColorType_Default") (InputField :type "EditableTextBox Object Reference"))
  (bind _returnvalue (`XsollaUIBuilderLibrary.GetTheme` Theme))
  (bind (_backgroundimagenormal _backgroundimagehovered _backgroundimagefocused _backgroundimagereadonly _padding _font _foregroundcolor _backgroundcolor _readonlyforegroundcolor _hscrollbarpadding _vscrollbarpadding _scrollbarstyle) (break `EditableTextBoxStyle` (`EditableTextBox.WidgetStyle` InputField)))
  (bind (_fontobject _fontmaterial _outlinesettings _typefacefontname _size _letterspacing) (break `SlateFontInfo` (`self.GetFont` Theme FontType (make `SlateFontInfo` "/Xsolla/Common/Assets/Font/Font_Roboto-Regular.Font_Roboto-Regular" null (struct :`OutlineColor` (struct :`A` 1.0)) "None" 14))))
  (`/Engine/EditorBlueprintResources/StandardMacros.IsValid` _returnvalue
    (:`Is Valid`
      (set `EditableTextBox.WidgetStyle` (make `EditableTextBoxStyle` (`XsollaUIBuilderTheme.GetBrushByType` _returnvalue NormalStateBrush) (`XsollaUIBuilderTheme.GetBrushByType` _returnvalue HoverStateBrush) (`XsollaUIBuilderTheme.GetBrushByType` _returnvalue ActiveStateBrush) (`XsollaUIBuilderTheme.GetBrushByType` _returnvalue DisabledStateBrush) _padding (make `SlateFontInfo` _fontobject _fontmaterial _outlinesettings _typefacefontname FontSize _letterspacing) (`self.GetColor` Theme TextColor (make `SlateColor` (struct :`R` 1.0 :`G` 1.0 :`B` 1.0 :`A` 0.7))) _backgroundcolor _readonlyforegroundcolor _hscrollbarpadding _vscrollbarpadding _scrollbarstyle) InputField))))