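; BP_FriendsItemData is a data object for a single friend entry in the Store demo.
; It wraps an ItemData record holding the user's ID and nickname along with incoming and outgoing status.
; Simple getters expose those fields and a stored Parent reference, with no other logic.
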(fn `GetIncomingStatus`
  (returns (IncomingStatus :type String))
  (return (`.status_incoming` (break `XsollaFriendDetails` (`self.ItemData`)))))

(fn `GetNickname`
  (returns (Nickname :type String))
  (return (`.nickname` (break `XsollaUserDetails` (`.user` (break `XsollaFriendDetails` (`self.ItemData`)))))))

(fn `GetOutgoingStatus`
  (returns (OutgoingStatus :type String))
  (return (`.status_outgoing` (break `XsollaFriendDetails` (`self.ItemData`)))))

(fn `GetParent`
  (returns (Parent :type "/Xsolla/NewDemo/Store/Interface/BPI_FriendsPanel Interface"))
  (return (`self.Parent`)))

(fn `GetUserID`
  (returns (UserID :type String))
  (return (`.id` (break `XsollaUserDetails` (`.user` (break `XsollaFriendDetails` (`self.ItemData`)))))))