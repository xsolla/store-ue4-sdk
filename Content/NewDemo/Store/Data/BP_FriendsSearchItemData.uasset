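; BP_FriendsSearchItemData is a data object for one user entry in a friends search, under the store demo.
; It wraps an ItemData record and exposes its user ID, nickname and avatar URL, along with a category.
; A RefreshIcon event stores the supplied icon and flags it as ready, which IsIconSet reports.
; GetParent returns no value.
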(event `/Xsolla/NewDemo/Store/Interface/BPI_IconPresenter.RefreshIcon`
  (params (Icon :type "SlateBrush Structure"))
  (set `self.Icon` Icon)
  (set `self.IsIconReady` true))

(fn `GetCategory`
  (returns (Category :type "/Xsolla/NewDemo/Store/Enum/UserFriendCategory Enum"))
  (return (`self.Category`)))

(fn `GetIcon`
  (returns (Icon :type "SlateBrush Structure"))
  (return (`self.Icon`)))

(fn `GetImageUrl`
  (returns (ImageUrl :type String))
  (return (`.avatar` (break `XsollaPublicProfile` (`self.ItemData`)))))

(fn `GetNickname`
  (returns (Nickname :type String))
  (return (`.nickname` (break `XsollaPublicProfile` (`self.ItemData`)))))

(fn `GetParent`
  (returns (Parent :type "/Xsolla/NewDemo/Store/Interface/BPI_FriendsPanel Interface"))
  (return null))

(fn `GetUserID`
  (returns (UserID :type String))
  (return (`.user_id` (break `XsollaPublicProfile` (`self.ItemData`)))))

(fn `IsIconSet`
  (returns (IsIconSet :type Boolean))
  (return (`self.IsIconReady`)))