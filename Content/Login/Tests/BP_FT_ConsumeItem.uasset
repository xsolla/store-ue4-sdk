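; Functional test that checks consuming an inventory item through the demo UI.
; It clicks the demo user login and Inventory buttons by widget name, then searches the inventory tile view for the item matching the virtual-purchase SKU.
; It consumes one unit, confirms the popup and passes if the message popup title reads "Success", with fixed delays between steps and explicit failures for missing panel, item or popups.
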(event `self.ReceiveTick`
  (params (DeltaSeconds :type "Float (single-precision)"))
  (`parent.ReceiveTick` DeltaSeconds))

(event `self.ReceiveStartTest`
  (bind _sku (`/Xsolla/Login/Tests/BPFL_LoginTests.GetBuyForVirtualSku`))
  (`parent.ReceiveStartTest`)
  (bind _returnvalue (`TestHelper.FindUIElementByName` "W_ButtonWrapper_DemoUser1" "/Xsolla/Common/Components/Wrappers/W_ButtonWrapper.W_ButtonWrapper_C"))
  (`/Xsolla/Common/Components/Wrappers/W_ButtonWrapper.OnClicked` _returnvalue)
  (`KismetSystemLibrary.Delay` 3.0)
  (bind _returnvalue_2 (`TestHelper.FindUIElementByName` "W_ButtonWrapper_Inventory" "/Xsolla/Common/Components/Wrappers/W_ButtonWrapper.W_ButtonWrapper_C"))
  (`/Xsolla/Common/Components/Wrappers/W_ButtonWrapper.OnClicked` _returnvalue_2)
  (`KismetSystemLibrary.Delay` 3.0)
  (bind _returnvalue_3 (`TestHelper.FindUIElementByName` "WidgetSwitcher_Main" "/Script/UMG.WidgetSwitcher"))
  (bind _returnvalue_4 (`WidgetSwitcher.GetActiveWidget` _returnvalue_3))
  (if (`KismetStringLibrary.EqualEqual_StrStr` (`KismetSystemLibrary.GetObjectName` _returnvalue_4) "W_InventoryPanel")
    (bind _asw_inventory_panel (cast `/Xsolla/Inventory/Panels/W_InventoryPanel` _returnvalue_4)
      (:`then`
        (for _array_element (`ListView.GetListItems` (`/Xsolla/Inventory/Panels/W_InventoryPanel.TileView_Inventory` _asw_inventory_panel))
          (bind _asbpi_inventory_item_data (cast `/Xsolla/Inventory/Interface/BPI_InventoryItemData` _array_element))
          (bind _sku_2 (`/Xsolla/Inventory/Interface/BPI_InventoryItemData.GetSku` _asbpi_inventory_item_data))
          (if (`KismetStringLibrary.EqualEqual_StrStr` _sku_2 _sku)
            (bind _instanceid (`/Xsolla/Inventory/Interface/BPI_InventoryItemData.GetInstanceId` _asbpi_inventory_item_data))
            (set `self.Instance Id` _instanceid)
            (set `self.bSkuWasFound` true)))
        (if (`self.bSkuWasFound`)
          (`/Xsolla/Inventory/Panels/W_InventoryPanel.ConsumeItem` _asw_inventory_panel _sku (`self.Instance Id`) 1)
          (`KismetSystemLibrary.Delay` 0.2)
          (bind _returnvalue_5 (`TestHelper.FindWidgetByClass` "/Xsolla/Common/Popup/W_ConfirmPopup.W_ConfirmPopup_C"))
          (`/Engine/EditorBlueprintResources/StandardMacros.IsValid` _returnvalue_5
            (:`Is Valid`
              (bind _returnvalue_6 (`TestHelper.FindUIElementInWidgetByName` _returnvalue_5 "W_ButtonWrapper_Confirm" "/Xsolla/Common/Components/Wrappers/W_ButtonWrapper.W_ButtonWrapper_C"))
              (`/Xsolla/Common/Components/Wrappers/W_ButtonWrapper.OnClicked` _returnvalue_6)
              (`KismetSystemLibrary.Delay` 3.0)
              (bind _returnvalue_7 (`TestHelper.FindWidgetByClass` "/Xsolla/Common/Popup/W_MessagePopup.W_MessagePopup_C"))
              (`/Engine/EditorBlueprintResources/StandardMacros.IsValid` _returnvalue_7
                (:`Is Valid`
                  (bind _returnvalue_8 (`TestHelper.FindUIElementInWidgetByName` _returnvalue_7 "W_TextWrapper_Title" "/Xsolla/Common/Components/Wrappers/W_TextWrapper.W_TextWrapper_C"))
                  (bind _text (`/Xsolla/Common/Components/Wrappers/W_TextWrapper.GetText` _returnvalue_8))
                  (`TestHelper.FinishTest` null (`KismetStringLibrary.EqualEqual_StrStr` (`KismetTextLibrary.Conv_TextToString` _text) "Success") "Success consume item!" "Item was not consumed"))
                (:`Is Not Valid`
                  (`self.FinishTest` "Failed" "Popup did not appear"))))
            (:`Is Not Valid`
              (`self.FinishTest` "Failed" "Confirm popup did not appear")))
          (else
            (`self.FinishTest` "Failed" (`KismetStringLibrary.Concat_StrStr` "Can't find item with sku " _sku)))))
      (:`CastFailed`
        (`self.FinishTest` "Failed" "W_InventoryPanel not opened" :!label _label)))
    (else
      (goto _label))))

(fn `UserConstructionScript`
  (`parent.UserConstructionScript`))