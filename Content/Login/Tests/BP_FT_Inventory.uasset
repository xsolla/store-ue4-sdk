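; Functional test Blueprint that checks the inventory panel loads after a demo user is selected.
; On start it finds UI buttons by name and fires their click handlers, DemoUser1 then Inventory, with fixed delays after each.
; It passes if the main widget switcher's active widget is the inventory panel, otherwise fails.
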(event `self.ReceiveTick`
  (params (DeltaSeconds :type "Float (single-precision)"))
  (`parent.ReceiveTick` DeltaSeconds))

(event `self.ReceiveStartTest`
  (`parent.ReceiveStartTest`)
  (bind _returnvalue (`TestHelper.FindUIElementByName` "W_ButtonWrapper_DemoUser1" "/Xsolla/Common/Components/Wrappers/W_ButtonWrapper.W_ButtonWrapper_C"))
  (`/Xsolla/Common/Components/Wrappers/W_ButtonWrapper.OnClicked` _returnvalue)
  (`KismetSystemLibrary.Delay` 3.0)
  (bind _returnvalue_2 (`TestHelper.FindUIElementByName` "W_ButtonWrapper_Inventory" "/Xsolla/Common/Components/Wrappers/W_ButtonWrapper.W_ButtonWrapper_C"))
  (`/Xsolla/Common/Components/Wrappers/W_ButtonWrapper.OnClicked` _returnvalue_2)
  (`KismetSystemLibrary.Delay` 3.0)
  (bind _returnvalue_3 (`TestHelper.FindUIElementByName` "WidgetSwitcher_Main" "/Script/UMG.WidgetSwitcher"))
  (`TestHelper.FinishTest` null (`KismetStringLibrary.EqualEqual_StrStr` (`KismetSystemLibrary.GetObjectName` (`WidgetSwitcher.GetActiveWidget` _returnvalue_3)) "W_InventoryPanel") "Success inventory loading" "Inventory was not loaded"))

(fn `UserConstructionScript`
  (`parent.UserConstructionScript`))