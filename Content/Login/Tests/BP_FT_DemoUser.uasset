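; Functional test that checks demo user login by clicking the first demo user button in the UI.
; On test start it finds the button widget by name and triggers its click, then waits a fixed delay.
; It passes if a store demo widget is found afterward and fails otherwise.
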(event `self.ReceiveStartTest`
  (`parent.ReceiveStartTest`)
  (bind _returnvalue (`TestHelper.FindUIElementByName` "W_Button_DemoUser1" "/Xsolla/Common/Components/Primitives/W_Button.W_Button_C"))
  (`/Xsolla/Common/Components/Primitives/W_Button.OnClicked` _returnvalue)
  (`KismetSystemLibrary.Delay` 3.0)
  (bind _returnvalue_2 (`TestHelper.FindWidgetByClass` "/Xsolla/Store/W_StoreDemo.W_StoreDemo_C"))
  (`TestHelper.FinishTest` null (`KismetSystemLibrary.IsValid` _returnvalue_2) "Success store login" "StoreWidget not found"))

(fn `UserConstructionScript`
  (`parent.UserConstructionScript`))