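; Functional test that checks Facebook social login in the Xsolla login demo, using an Email and Password set on the placed instance.
; It clicks the Facebook icon button, then injects JavaScript into the Xsolla web browser to fill and submit the login form.
; After fixed delays it passes if the store demo widget exists, and fails early without an Email.
; An unused keyboard-typing path remains, noted as crash-prone from unstable browser focus.
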(event `self.ReceiveStartTest`
  (`parent.ReceiveStartTest`)
  (if (not (`KismetStringLibrary.IsEmpty` (`self.Email`)))
    (bind _returnvalue (`TestHelper.FindUIElementByName` "W_IconButton_Facebook1" "/Xsolla/Common/Components/Primitives/W_IconButton.W_IconButton_C"))
    (`/Xsolla/Common/Components/Primitives/W_IconButton.OnIconButtonClicked` _returnvalue)
    (`KismetSystemLibrary.Delay` 5.0)
    (bind _returnvalue_2 (`TestHelper.FindUIElementByName` "XsollaWebBrowser_43" "/Script/XsollaWebBrowser.XsollaWebBrowser"))
    (`XsollaWebBrowser.ExecuteJavascript` _returnvalue_2 (`KismetTextLibrary.Conv_TextToString` (`|FormatText` "document.querySelector(\"input[id='email']\").value = \"{Email}\"" (`self.Email`))))
    (`XsollaWebBrowser.ExecuteJavascript` _returnvalue_2 (`KismetTextLibrary.Conv_TextToString` (`|FormatText` "document.querySelector(\"input[id='pass']\").value = \"{Password}\"" (`self.Password`))))
    (`XsollaWebBrowser.ExecuteJavascript` _returnvalue_2 "document.querySelector(\"button[id='loginbutton']\").click()")
    (`KismetSystemLibrary.Delay` 10.0)
    (bind _returnvalue_3 (`TestHelper.FindWidgetByClass` "/Xsolla/Store/W_StoreDemo.W_StoreDemo_C"))
    (`TestHelper.FinishTest` null (`KismetSystemLibrary.IsValid` _returnvalue_3) "Success" "Failed")
    (else
      (`TestHelper.FinishTest` null false "" "Missed Email at Test - setup at Scene for this instance"))))

(fn `UserConstructionScript`
  (`parent.UserConstructionScript`))