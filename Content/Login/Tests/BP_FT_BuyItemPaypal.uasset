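; Functional test that checks buying a real-money store item through PayPal in the Xsolla payment browser.
; It drives the UI by widget name to sign in as a demo user, open the store and purchase the configured SKU.
; Fixed delays pace injected JavaScript clicks through the checkout page.
; It passes when the message popup confirms the order, and fails on a wrong panel, missing SKU, absent popup or different message.
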(event `self.ReceiveStartTest`
  (bind _sku (`/Xsolla/Login/Tests/BPFL_LoginTests.GetBuyForRealSku`))
  (`parent.ReceiveStartTest`)
  (bind _returnvalue (`TestHelper.FindUIElementByName` "W_ButtonWrapper_DemoUser1" "/Xsolla/Common/Components/Wrappers/W_ButtonWrapper.W_ButtonWrapper_C"))
  (`/Xsolla/Common/Components/Wrappers/W_ButtonWrapper.OnClicked` _returnvalue)
  (`KismetSystemLibrary.Delay` 3.0)
  (bind _returnvalue_2 (`TestHelper.FindUIElementByName` "W_ButtonWrapper_Store" "/Xsolla/Common/Components/Wrappers/W_ButtonWrapper.W_ButtonWrapper_C"))
  (`/Xsolla/Common/Components/Wrappers/W_ButtonWrapper.OnClicked` _returnvalue_2)
  (`KismetSystemLibrary.Delay` 5.0)
  (bind _returnvalue_3 (`TestHelper.FindUIElementByName` "WidgetSwitcher_Main" "/Script/UMG.WidgetSwitcher"))
  (bind _returnvalue_4 (`WidgetSwitcher.GetActiveWidget` _returnvalue_3))
  (if (`KismetStringLibrary.EqualEqual_StrStr` (`KismetSystemLibrary.GetObjectName` _returnvalue_4) "W_StorePanel_Items")
    (bind _asw_store_panel (cast `/Xsolla/Store/Panels/W_StorePanel` _returnvalue_4)
      (:`then`
        (for _array_element (`ListView.GetListItems` (`/Xsolla/Store/Panels/W_StorePanel.TileView_Store` _asw_store_panel))
          (bind _asbpi_store_item_data (cast `/Xsolla/Store/Interface/BPI_StoreItemData` _array_element))
          (bind _sku_2 (`/Xsolla/Store/Interface/BPI_StoreItemData.GetSku` _asbpi_store_item_data))
          (if (`KismetStringLibrary.EqualEqual_StrStr` _sku_2 _sku)
            (set `self.bSkuWasFound` true)))
        (if (`self.bSkuWasFound`)
          (`/Xsolla/Store/Panels/W_StorePanel.PurchaseItem` _asw_store_panel _sku)
          (`KismetSystemLibrary.Delay` 5.0)
          (bind _returnvalue_5 (`TestHelper.FindUIElementByName` "XsollaWebBrowser_Browser" "/Script/XsollaWebBrowser.XsollaWebBrowser"))
          (`XsollaWebBrowser.ExecuteJavascript` _returnvalue_5 "document.querySelector(\"div[title='PayPal']\").click()")
          (`KismetSystemLibrary.Delay` 5.0)
          (`XsollaWebBrowser.ExecuteJavascript` _returnvalue_5 "document.querySelector(\"button[class='btn btn-md btn-flat btn-accent']\").click()")
          (`KismetSystemLibrary.Delay` 5.0)
          (`XsollaWebBrowser.ExecuteJavascript` _returnvalue_5 "document.querySelector(\"button[class='btn btn-md btn-flat btn-accent']\").click()")
          (`KismetSystemLibrary.Delay` 5.0)
          (`XsollaWebBrowser.ExecuteJavascript` _returnvalue_5 "document.querySelector(\"a[class='btn btn-flat btn-md btn-accent tab-focus']\").click()")
          (`KismetSystemLibrary.Delay` 7.0)
          (bind _foundwidgets (`WidgetBlueprintLibrary.GetAllWidgetsOfClass` "/Xsolla/Common/Popup/W_MessagePopup.W_MessagePopup_C"))
          (if (`KismetArrayLibrary.Array_IsValidIndex` _foundwidgets)
            (bind _returnvalue_6 (`TestHelper.FindUIElementInWidgetByName` (`|GetArrayItem` _foundwidgets) "W_TextWrapper_Message" "/Xsolla/Common/Components/Wrappers/W_TextWrapper.W_TextWrapper_C"))
            (bind _text (`/Xsolla/Common/Components/Wrappers/W_TextWrapper.GetText` _returnvalue_6))
            (`TestHelper.FinishTest` null (`KismetStringLibrary.EqualEqual_StrStr` (`KismetTextLibrary.Conv_TextToString` _text) "Your order has been successfully processed!") "Successfull purchase!" "Item was not purchased")
            (else
              (`self.FinishTest` "Failed" "Popup did not appear")))
          (else
            (`self.FinishTest` "Failed" (`KismetStringLibrary.Concat_StrStr` "Can't find item with sku " _sku)))))
      (:`CastFailed`
        (`self.FinishTest` "Failed" "W_StorePanel_Items not opened" :!label _label)))
    (else
      (goto _label))))

(fn `GetQueryString`
  (params (type :type String) (id :type String) (value :type String))
  (returns (result :type String))
  (return (`KismetTextLibrary.Conv_TextToString` (`|FormatText` "document.querySelector(\"{type}[id='{Id}']\").value = \"{Value}\"" type id value))))

(fn `UserConstructionScript`
  (`parent.UserConstructionScript`))