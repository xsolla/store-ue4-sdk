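; BP_FT_BasicAuth is a functional test for basic login that checks whether authentication leads to the store demo screen.
; On test start it calls MakeLogin with hardcoded credentials, waits a fixed delay, then searches for a W_StoreDemo widget.
; The test passes if that widget is valid, relying on timing and UI presence rather than a login callback.
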(event `self.ReceiveStartTest`
  (`parent.ReceiveStartTest`)
  (`/Xsolla/Login/Tests/BPFL_LoginTests.MakeLogin` "xsolla" "xsolla")
  (`KismetSystemLibrary.Delay` 3.0)
  (bind _returnvalue (`TestHelper.FindWidgetByClass` "/Xsolla/Store/W_StoreDemo.W_StoreDemo_C"))
  (`TestHelper.FinishTest` null (`KismetSystemLibrary.IsValid` _returnvalue) "Success store login" "StoreWidget not found"))

(fn `UserConstructionScript`
  (`parent.UserConstructionScript`))