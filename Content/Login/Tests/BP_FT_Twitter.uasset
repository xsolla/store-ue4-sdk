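; BP_FT_Twitter is a functional test of the Twitter login flow, run with an Email and Password set on the scene instance.
; It clicks the Twitter button, then injects JavaScript into the Xsolla web browser widget to fill and submit the form.
; After fixed delays it passes if a W_StoreDemo widget exists, and fails if Email is empty.
; An unused simulated-typing path remains, noted as crash-prone due to unstable browser focus.
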(event `self.ReceiveStartTest`
  (`parent.ReceiveStartTest`)
  (if (not (`KismetStringLibrary.IsEmpty` (`self.Email`)))
    (bind _returnvalue (`TestHelper.FindUIElementByName` "W_ButtonWrapper_Twitter1" "/Xsolla/Common/Components/Wrappers/W_ButtonWrapper.W_ButtonWrapper_C"))
    (`/Xsolla/Common/Components/Wrappers/W_ButtonWrapper.OnClicked` _returnvalue)
    (`KismetSystemLibrary.Delay` 5.0)
    (bind _returnvalue_2 (`TestHelper.FindUIElementByName` "XsollaWebBrowser_43" "/Script/XsollaWebBrowser.XsollaWebBrowser"))
    (`XsollaWebBrowser.ExecuteJavascript` _returnvalue_2 (`KismetTextLibrary.Conv_TextToString` (`|FormatText` "document.querySelector(\"input[id='username_or_email']\").value = \"{Email}\"" (`self.Email`))))
    (`XsollaWebBrowser.ExecuteJavascript` _returnvalue_2 (`KismetTextLibrary.Conv_TextToString` (`|FormatText` "document.querySelector(\"input[id='password']\").value = \"{Password}\"" (`self.Password`))))
    (`XsollaWebBrowser.ExecuteJavascript` _returnvalue_2 "document.querySelector(\"input[id='allow']\").click()")
    (`KismetSystemLibrary.Delay` 10.0)
    (bind _returnvalue_3 (`TestHelper.FindWidgetByClass` "/Xsolla/Store/W_StoreDemo.W_StoreDemo_C"))
    (`TestHelper.FinishTest` null (`KismetSystemLibrary.IsValid` _returnvalue_3) "Success" "Failed")
    (else
      (`TestHelper.FinishTest` null false "" "Missed Email at Test - setup at Scene for this instance"))))

(fn `UserConstructionScript`
  (`parent.UserConstructionScript`))