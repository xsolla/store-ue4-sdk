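; Functional test that checks new-account registration through the login UI.
; On start it builds a unique account name from the Unix timestamp, finds widgets by name, opens sign-up, fills the username, email and password fields, and clicks create.
; After a fixed delay, it passes only if the popup title reads as a successful account creation, so it depends on exact widget names and message text.
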(event `self.ReceiveStartTest`
  (`parent.ReceiveStartTest`)
  (set `self.AccountName` (`KismetStringLibrary.Concat_StrStr` "SDKUnrealTestAccount" (`KismetTextLibrary.Conv_TextToString` (`KismetTextLibrary.Conv_Int64ToText` (`XsollaUtilsLibrary.GetSecondsFromUnixTimestamp` (`KismetMathLibrary.UtcNow`)) false false))))
  (bind _returnvalue (`TestHelper.FindUIElementByName` "W_Button_OpenSignUp" "/Xsolla/Common/Components/Primitives/W_Button.W_Button_C"))
  (`/Xsolla/Common/Components/Primitives/W_Button.OnClicked` _returnvalue)
  (`TestHelper.SetInputFieldText` "W_Input_NewUsername" (`KismetTextLibrary.Conv_StringToText` (`self.AccountName`)) true)
  (`TestHelper.SetInputFieldText` "W_Input_NewEmail" (`|FormatText` "{AccountName}@qwemail.com" (`self.AccountName`)) true)
  (`TestHelper.SetInputFieldText` "W_Input_NewPassword" (`KismetTextLibrary.Conv_StringToText` (`self.AccountName`)) true)
  (bind _returnvalue_2 (`TestHelper.FindUIElementByName` "W_Button_CreateAccount" "/Xsolla/Common/Components/Primitives/W_Button.W_Button_C"))
  (`/Xsolla/Common/Components/Primitives/W_Button.OnClicked` _returnvalue_2)
  (`KismetSystemLibrary.Delay` 3.0)
  (bind _returnvalue_3 (`TestHelper.FindUIElementByName` "TextBlock_PopupMessageTitle" "/Script/UMG.TextBlock"))
  (`TestHelper.FinishTest` null (`KismetTextLibrary.EqualEqual_TextText` (`TextBlock.GetText` _returnvalue_3) "Account successfully created") "Account successfully created." "Account not created."))

(fn `UserConstructionScript`
  (`parent.UserConstructionScript`))