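; Login-area icon loader that fetches images by URL and applies them to icon presenters.
; LoadIcons adds presenters to a pending cache, clearing it first only if every icon is set, then requests an image for each cached entry.
; Success and error callbacks refresh every cached presenter with a matching URL, using a not-loaded placeholder texture on failure.
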(event `/Xsolla/Login/Interface/BPI_IconsLoader.LoadIcons`
  (params (IconPresentersData :type "Array of /Xsolla/Common/Interface/BPI_IconPresenter Interface (by ref)"))
  ;[1 1 1] LoadIcons
  (if (not (`self.CheckForPendingIcons`))
    (`KismetArrayLibrary.Array_Clear` (`self.PendingIconsCache`)))
  (`KismetArrayLibrary.Array_Append` (`self.PendingIconsCache`) IconPresentersData)
  (for _array_element (`self.PendingIconsCache`)
    (bind _imageurl (`/Xsolla/Common/Interface/BPI_IconPresenter.GetImageUrl` _array_element))
    (`XsollaUtilsImageLoader.LoadImage` (`XsollaUtilsLibrary.GetImageLoader`) _imageurl (delegate `OnImageLoadSuccess`) (delegate `OnImageLoadError`))))

(event `OnImageLoadSuccess`
  (params (ImageBrush :type "SlateBrush Structure") (ImageURL :type String))
  ;[1 1 1] LoadIcons
  (`self.UpdateProperIconPresenters` (`self.PendingIconsCache`) ImageURL ImageBrush))

(event `OnImageLoadError`
  (params (ImageURL :type String))
  ;[1 1 1] LoadIcons
  (`self.UpdateProperIconPresenters` (`self.PendingIconsCache`) ImageURL (`WidgetBlueprintLibrary.MakeBrushFromTexture` "/Xsolla/Common/Assets/Icon/T_Icon_NotLoaded.T_Icon_NotLoaded" 100 100) true))

(fn `CheckForPendingIcons`
  (returns (PendingIconsExist :type Boolean))
  (for _array_element (`self.PendingIconsCache`)
    (bind _isiconset (`/Xsolla/Common/Interface/BPI_IconPresenter.IsIconSet` _array_element))
    (if (not _isiconset)
      (return true)))
  (return false))

(fn `UpdateProperIconPresenters`
  (params (IconPresenters :type "Array of /Xsolla/Common/Interface/BPI_IconPresenter Interface (by ref)") (ImageURL :type String) (Icon :type "SlateBrush Structure") (IsError :type Boolean))
  (for _array_element IconPresenters
    (bind _imageurl (`/Xsolla/Common/Interface/BPI_IconPresenter.GetImageUrl` _array_element))
    (if (`KismetStringLibrary.EqualEqual_StrStr` _imageurl ImageURL)
      (`/Xsolla/Common/Interface/BPI_IconPresenter.RefreshIcon` _array_element (select `bool` IsError :`false` Icon :`true` (`WidgetBlueprintLibrary.MakeBrushFromTexture` "/Xsolla/Common/Assets/Icon/T_Icon_NotLoaded.T_Icon_NotLoaded" 100 100))))))