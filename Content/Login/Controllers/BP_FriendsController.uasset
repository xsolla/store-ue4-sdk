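; Controller for the Xsolla Login demo's friends screen, handling friend lists, nickname search, social network linking and friend actions through the Xsolla Login subsystem.
; A refresh fires parallel requests and redraws the panel once ready flags and a game-profile countdown show all are done.
; Results become item-data objects with loaded icons; social friends and search results are filtered by existing relationship.
; Removing or blocking requires popup confirmation, and successful actions refresh the panel.
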(event `self.OnSocialNetworkLinkingInitiated`
  (params (Provider :type String) (Panel :type "/Xsolla/Login/Interface/BPI_FriendsPanel Interface"))
  ;[1 1 1] Link social network account
  (`/Xsolla/Common/BP_DemoUtils.ShowLoader` true)
  (`XsollaLoginSubsystem.LinkSocialNetworkToUserAccount` (subsystem `XsollaLoginSubsystem`) (`self.GetToken`) Provider (delegate `OnSocialNetworkLinkSuccess`) (`|CreateDelegate` :!event `ShowLoginError`)))

(event `OnSocialNetworkLinkSuccess`
  (params (Content :type String))
  ;[1 1 1] Link social network account
  (`/Xsolla/Common/BP_DemoUtils.ShowLoader` false)
  (bind _returnvalue (`|CreateWidget` "/Xsolla/Login/Components/W_LoginBrowserLinking.W_LoginBrowserLinking_C" (`GameplayStatics.GetPlayerController` 0) Content))
  (add `/Xsolla/Login/Components/W_LoginBrowserLinking.Browser Closed` _returnvalue (delegate `OnLinkingBrowserClosed`))
  (`UserWidget.AddToViewport` _returnvalue 10000))

(event `OnLinkingBrowserClosed`
  ;[1 1 1] Link social network account
  (`/Xsolla/Common/BP_DemoUtils.ShowLoader` true)
  (`XsollaLoginSubsystem.UpdateUsersFriends` (subsystem `XsollaLoginSubsystem`) (`self.GetToken`) (stale `self.OnSocialNetworkLinkingInitiated` Provider) (delegate `OnUpdateUsersFriendsSuccess`) (`|CreateDelegate` :!event `ShowLoginError`)))

(event `OnUpdateUsersFriendsSuccess`
  (params (Code :type String))
  ;[1 1 1] Link social network account
  (`/Xsolla/Common/BP_DemoUtils.ShowLoader` false)
  (`self.RefreshFriendsPanel` true (stale `self.OnSocialNetworkLinkingInitiated` Panel)))

(event `self.RefreshFriendsPanel`
  (params (Redraw :type Boolean) (Panel :type "/Xsolla/Login/Interface/BPI_FriendsPanel Interface"))
  ;[1 1 1] Refresh friends panel
  (`KismetArrayLibrary.Array_Clear` (`self.Friends`))
  (`/Xsolla/Common/BP_DemoUtils.ShowLoader` true)
  (`self.ResetFriendsRequestsFlags`)
  (bind _keys (`BlueprintMapLibrary.Map_Keys` (`self.FriendsRequestsReady`)))
  (for _array_element _keys
    (`XsollaLoginSubsystem.UpdateFriends` (subsystem `XsollaLoginSubsystem`) (`self.GetToken`) _array_element "by_nickname" "asc" (delegate `OnFriendsUpdateSuccess`) (`|CreateDelegate` :!event `ShowLoginError`) "" 20))
  (set `self.SocialNetworksStatusReady` false)
  (`XsollaLoginSubsystem.UpdateLinkedSocialNetworks` (subsystem `XsollaLoginSubsystem`) (`self.GetToken`) (delegate `OnLinkedSocialNetworksUpdateSuccess`) (`|CreateDelegate` :!event `ShowLoginError`))
  (set `self.SocialFriendsStatusReady` false)
  (`XsollaLoginSubsystem.UpdateSocialFriends` (subsystem `XsollaLoginSubsystem`) (`self.GetToken`) "" (delegate `OnUpdateSocialFriendsCompleted`) (`|CreateDelegate` :!event `ShowLoginError`) 0 500 false))

(event `OnUpdateSocialFriendsCompleted`
  (params (SocialFriendsData :type "XsollaSocialFriendsData Structure (by ref)"))
  ;[1 1 1] Refresh friends panel
  (`self.GetSocialFriendsGameProfileData`))

(event `OnLinkedSocialNetworksUpdateSuccess`
  ;[1 1 1] Refresh friends panel
  (set `self.SocialNetworksStatusReady` true)
  (if (and (`self.FriendsRequestReady`) (`self.SocialNetworksStatusReady`) (`self.SocialFriendsStatusReady`)) :!label _label
    (`/Xsolla/Common/BP_DemoUtils.ShowLoader` false)
    (`/Xsolla/Login/Interface/BPI_FriendsPanel.RefreshFriendsList` (stale `self.RefreshFriendsPanel` Panel) (`self.Friends`) (stale `self.RefreshFriendsPanel` Redraw))
    (bind _socialnetworks (`self.CreateSocialNetworksData` (stale `self.RefreshFriendsPanel` Panel)))
    (`/Xsolla/Login/Interface/BPI_FriendsPanel.RefreshSocialNetworksList` (stale `self.RefreshFriendsPanel` Panel) _socialnetworks)
    (bind _friends (`self.CreateSocialFriendsData` (stale `self.RefreshFriendsPanel` Panel)))
    (`/Xsolla/Login/Interface/BPI_FriendsPanel.RefreshSocialFriendsList` (stale `self.RefreshFriendsPanel` Panel) _friends (stale `self.RefreshFriendsPanel` Redraw))
    (`/Xsolla/Login/Interface/BPI_DemoWidget.ActivateFriendsPanel` (`self.DemoWidget`))))

(event `OnSocialFriendsStatusUpdate`
  ;[1 1 1] Refresh friends panel
  (goto _label))

(event `OnFriendsUpdateSuccess`
  (params (FriendsData :type "XsollaFriendsData Structure (by ref)") (type :type "EXsollaFriendsType Enum" :default "friends"))
  ;[1 1 1] Refresh friends panel
  (`BlueprintMapLibrary.Map_Add` (`self.FriendsRequestsReady`) type true)
  (bind _friends (`self.CreateFriendsData` FriendsData (stale `self.RefreshFriendsPanel` Panel)))
  (`KismetArrayLibrary.Array_Append` (`self.Friends`) _friends)
  (goto _label))

(event `self.OnUserSearchInitiated`
  (params (Nickname :type String) (Panel :type "/Xsolla/Login/Interface/BPI_FriendsPanel Interface"))
  ;[1 1 1] Search user by nickname
  (`/Xsolla/Common/BP_DemoUtils.ShowLoader` true)
  (`XsollaLoginSubsystem.SearchUsersByNickname` (subsystem `XsollaLoginSubsystem`) (`self.GetToken`) Nickname (delegate `OnSearchUsersSuccess`) (`|CreateDelegate` :!event `ShowLoginError`) 0 100))

(event `OnSearchUsersSuccess`
  (params (SearchResult :type "XsollaUserSearchResult Structure (by ref)"))
  ;[1 1 1] Search user by nickname
  (`/Xsolla/Common/BP_DemoUtils.ShowLoader` false)
  (bind _friendssearchdata (`self.CreateFriendsSearchData` SearchResult (stale `self.OnUserSearchInitiated` Panel)))
  (`/Xsolla/Login/Interface/BPI_FriendsPanel.RefreshFriendsSearchList` (stale `self.OnUserSearchInitiated` Panel) _friendssearchdata))

(event `self.OnUserActionInitiated`
  (params (UserId :type String) (Action :type "/Xsolla/Login/Enum/UserActionType Enum" :default "NewEnumerator0") (Nickname :type String) (Panel :type "/Xsolla/Login/Interface/BPI_FriendsPanel Interface"))
  (bind (_message _confirmbuttontext) (`self.FormatActionConfirmationMessage` Action Nickname))
  ;[1 1 1] Perform user action
  (if (`self.UserActionRequiresConfirmation` Action)
    (bind _returnvalue (`|CreateWidget` "/Xsolla/Common/Popup/W_ConfirmPopup.W_ConfirmPopup_C" (`GameplayStatics.GetPlayerController` 0) _message _confirmbuttontext))
    (`UserWidget.AddToViewport` _returnvalue 10000)
    (add `/Xsolla/Common/Popup/W_ConfirmPopup.OnPopupResult` _returnvalue (delegate `OnUserActionConfirmed`))
    (else
      (`/Xsolla/Common/BP_DemoUtils.ShowLoader` true :!label _label_2)
      (`XsollaLoginSubsystem.ModifyFriends` (subsystem `XsollaLoginSubsystem`) (`self.GetToken`) (`self.ConvertActionEnum` Action) UserId (delegate `OnUserUnblockSuccess`) (`|CreateDelegate` :!event `ShowLoginError`)))))

(event `OnUserActionConfirmed`
  (params (IsConfirmed :type Boolean))
  ;[1 1 1] Perform user action
  (if IsConfirmed
    (goto _label_2)))

(event `OnUserUnblockSuccess`
  ;[1 1 1] Perform user action
  (`/Xsolla/Common/BP_DemoUtils.ShowLoader` false)
  (`self.RefreshFriendsPanel` false (stale `self.OnUserActionInitiated` Panel))
  (`/Xsolla/Login/Interface/BPI_FriendsPanel.HandleUserActionUpdate` (stale `self.OnUserActionInitiated` Panel) (stale `self.OnUserActionInitiated` UserId)))

(fn `ConvertActionEnum`
  (params (Index :type "/Xsolla/Login/Enum/UserActionType Enum" :default "NewEnumerator0"))
  (returns (ReturnValue :type "EXsollaFriendAction Enum"))
  (return (select `/Xsolla/Login/Enum/UserActionType` Index :`NewEnumerator0` "friend_request_add" :`NewEnumerator1` "friend_request_cancel" :`NewEnumerator4` "friend_request_approve" :`NewEnumerator5` "friend_request_deny" :`NewEnumerator2` "block" :`NewEnumerator3` "unblock" :`NewEnumerator6` "friend_remove" :!type "EXsollaFriendAction Enum")))

(fn `CreateFriendsData`
  (params (FriendsData :type "XsollaFriendsData Structure (by ref)") (Panel :type "/Xsolla/Login/Interface/BPI_FriendsPanel Interface"))
  (returns (Friends :type "Array of /Xsolla/Login/Interface/BPI_FriendsItemData Interface"))
  (locals (FriendsArray :type "Array of /Xsolla/Login/Interface/BPI_FriendsItemData Interface") (IconPresenters :type "Array of /Xsolla/Common/Interface/BPI_IconPresenter Interface"))
  (for _array_element (`.relationships` (break `XsollaFriendsData` FriendsData))
    (bind _returnvalue (`|GenericCreateObject` "/Xsolla/Login/Data/BP_FriendsItemData.BP_FriendsItemData_C" self _array_element Panel))
    (`KismetArrayLibrary.Array_Add` (`local.FriendsArray`) _returnvalue)
    (`KismetArrayLibrary.Array_Add` (`local.IconPresenters`) _returnvalue))
  (`/Xsolla/Login/Interface/BPI_Demo.LoadIcons` (`self.Demo`) (`local.IconPresenters`))
  (return (`local.FriendsArray`)))

(fn `CreateFriendsSearchData`
  (params (SearchResult :type "XsollaUserSearchResult Structure (by ref)") (Parent :type "/Xsolla/Login/Interface/BPI_FriendsPanel Interface"))
  (returns (FriendsSearchData :type "Array of /Xsolla/Login/Interface/BPI_FriendsSearchItemData Interface"))
  (locals (SearchData :type "Array of /Xsolla/Login/Interface/BPI_FriendsSearchItemData Interface") (IconPresenters :type "Array of /Xsolla/Common/Interface/BPI_IconPresenter Interface"))
  (for _array_element (`.users` (break `XsollaUserSearchResult` SearchResult))
    (bind (_avatar _is_me _last_login _nickname _tag _registered _user_id) (break `XsollaPublicProfile` _array_element))
    (bind _category (`self.GetUserRelations` _user_id))
    (if (not (`self.Ignore Search Result` _category))
      (bind _returnvalue (`|GenericCreateObject` "/Xsolla/Login/Data/BP_FriendsSearchItemData.BP_FriendsSearchItemData_C" self Parent _array_element _category (`XsollaLoginSubsystem.GetSocialProfiles` (subsystem `XsollaLoginSubsystem`) _user_id)))
      (`KismetArrayLibrary.Array_Add` (`local.SearchData`) _returnvalue)
      (`KismetArrayLibrary.Array_Add` (`local.IconPresenters`) _returnvalue)))
  (`/Xsolla/Login/Interface/BPI_Demo.LoadIcons` (`self.Demo`) (`local.IconPresenters`))
  (return (`local.SearchData`)))

(fn `CreateSocialFriendsData`
  (params (FriendsPanel :type "/Xsolla/Login/Interface/BPI_FriendsPanel Interface"))
  (returns (Friends :type "Array of /Xsolla/Login/Interface/BPI_FriendsSocialItemData Interface"))
  (locals (SocialFriendsArray :type "Array of /Xsolla/Login/Interface/BPI_FriendsSocialItemData Interface") (IconPresenters :type "Array of /Xsolla/Common/Interface/BPI_IconPresenter Interface"))
  (bind _keys (`BlueprintMapLibrary.Map_Keys` (`self.SocialFriendsGameProfiles`)))
  (for _array_element _keys
    (bind _category (`self.GetUserRelations` _array_element))
    (if (`self.IsValidFriendRecommendation` _category)
      (bind _returnvalue (`|GenericCreateObject` "/Xsolla/Login/Data/BP_FriendsSocialItemData.BP_FriendsSocialItemData_C" self FriendsPanel (`XsollaLoginSubsystem.GetSocialProfiles` (subsystem `XsollaLoginSubsystem`) _array_element) _category (`BlueprintMapLibrary.Map_Find` (`self.SocialFriendsGameProfiles`) _array_element)))
      (`KismetArrayLibrary.Array_Add` (`local.SocialFriendsArray`) _returnvalue)
      (`KismetArrayLibrary.Array_Add` (`local.IconPresenters`) _returnvalue)))
  (for _array_element_2 (`.data` (break `XsollaSocialFriendsData` (`XsollaLoginSubsystem.GetSocialFriends` (subsystem `XsollaLoginSubsystem`))))
    (if (== (`KismetStringLibrary.Len` (`.xl_uid` (break `XsollaSocialFriend` _array_element_2))) 0)
      (bind _returnvalue_2 (`|GenericCreateObject` "/Xsolla/Login/Data/BP_FriendsSocialItemData.BP_FriendsSocialItemData_C" self FriendsPanel (`|MakeArray` _array_element_2) "NewEnumerator5"))
      (`KismetArrayLibrary.Array_Add` (`local.SocialFriendsArray`) _returnvalue_2)
      (`KismetArrayLibrary.Array_Add` (`local.IconPresenters`) _returnvalue_2)))
  (`/Xsolla/Login/Interface/BPI_Demo.LoadIcons` (`self.Demo`) (`local.IconPresenters`))
  (return (`local.SocialFriendsArray`)))

(fn `CreateSocialNetworksData`
  (params (FriendsPanel :type "/Xsolla/Login/Interface/BPI_FriendsPanel Interface"))
  (returns (SocialNetworks :type "Array of /Xsolla/Login/Interface/BPI_SocialNetworkItemData Interface"))
  (locals (Networks :type "Array of /Xsolla/Login/Interface/BPI_SocialNetworkItemData Interface"))
  (bind _keys (`BlueprintMapLibrary.Map_Keys` (`self.SocialNetworks`)))
  (for _array_element _keys
    (bind _returnvalue (`|GenericCreateObject` "/Xsolla/Login/Data/BP_SocialNetworkItemData.BP_SocialNetworkItemData_C" self (`XsollaLoginSubsystem.IsSocialNetworkLinked` (subsystem `XsollaLoginSubsystem`) _array_element) _array_element (`BlueprintMapLibrary.Map_Find` (`self.SocialNetworks`) _array_element) FriendsPanel))
    (`KismetArrayLibrary.Array_Add` (`local.Networks`) _returnvalue))
  (return (`local.Networks`)))

(fn `FormatActionConfirmationMessage`
  (params (Action :type "/Xsolla/Login/Enum/UserActionType Enum" :default "NewEnumerator0") (Nickname :type String))
  (returns (Message :type Text) (ConfirmButtonText :type Text))
  (return (select `/Xsolla/Login/Enum/UserActionType` Action :`NewEnumerator2` (`|FormatText` "Block {Nickname}?" Nickname) :`NewEnumerator6` (`|FormatText` "Remove {Nickname} from the friends list?" Nickname)) (select `/Xsolla/Login/Enum/UserActionType` Action :`NewEnumerator2` "BLOCK" :`NewEnumerator6` "REMOVE" :!type "Text")))

(fn `FriendsRequestReady`
  (returns (Ready :type Boolean))
  (bind _keys (`BlueprintMapLibrary.Map_Keys` (`self.FriendsRequestsReady`)))
  (for _array_element _keys
    (if (not (`BlueprintMapLibrary.Map_Find` (`self.FriendsRequestsReady`) _array_element))
      (return false)))
  (return true))

(fn `GetSocialFriendsGameProfileData`
  (locals (UsersWithGameProfile :type "Array of XsollaSocialFriend Structure"))
  (bind _returnvalue (`KismetArrayLibrary.Array_Length` (`local.UsersWithGameProfile`)))
  (`BlueprintMapLibrary.Map_Clear` (`self.SocialFriendsGameProfiles`))
  (for _array_element (`.data` (break `XsollaSocialFriendsData` (`XsollaLoginSubsystem.GetSocialFriends` (subsystem `XsollaLoginSubsystem`))))
    (if (> (`KismetStringLibrary.Len` (`.xl_uid` (break `XsollaSocialFriend` _array_element))) 0)
      (`KismetArrayLibrary.Array_Add` (`local.UsersWithGameProfile`) _array_element)))
  (set `self.RemainingGameProfileRequests` _returnvalue)
  (if (> _returnvalue 0)
    (for _array_element_2 (`local.UsersWithGameProfile`)
      (`XsollaLoginSubsystem.GetUserProfile` (subsystem `XsollaLoginSubsystem`) (`self.GetToken`) (`.xl_uid` (break `XsollaSocialFriend` _array_element_2)) (`|CreateDelegate` :!event `Handle Social Friend Game Profile Request`) (`|CreateDelegate` :!event `ShowLoginError`)))
    (else
      (set `self.SocialFriendsStatusReady` true)
      (`self.OnSocialFriendsStatusUpdate`))))

(fn `GetToken`
  (returns (Token :type String))
  (return (`.JWT` (break `XsollaAuthToken` (`.AuthToken` (break `XsollaLoginData` (`XsollaLoginSubsystem.GetLoginData` (subsystem `XsollaLoginSubsystem`))))))))

(fn `GetUserRelations`
  (params (UserId :type String))
  (returns (Category :type "/Xsolla/Login/Enum/UserFriendCategory Enum"))
  (for _array_element (`self.Friends`)
    (bind _userid (`/Xsolla/Login/Interface/BPI_FriendsItemData.GetUserID` _array_element))
    (bind _category (`/Xsolla/Login/Interface/BPI_FriendsItemData.GetCategory` _array_element))
    (if (`KismetStringLibrary.EqualEqual_StrStr` _userid UserId)
      (return _category)))
  (return "NewEnumerator5"))

(fn `Handle Social Friend Game Profile Request`
  (params (UserProfile :type "XsollaPublicProfile Structure (by ref)"))
  (`BlueprintMapLibrary.Map_Add` (`self.SocialFriendsGameProfiles`) (`.user_id` (break `XsollaPublicProfile` UserProfile)))
  (set `self.RemainingGameProfileRequests` (- (`self.RemainingGameProfileRequests`) 1))
  (set `self.SocialFriendsStatusReady` (== (`self.RemainingGameProfileRequests`) 0))
  (`self.OnSocialFriendsStatusUpdate`))

(fn `Ignore Search Result`
  (params (Category :type Byte))
  (returns (ShouldIgnore :type Boolean))
  (return (or (== Category (enumliteral `/Xsolla/Login/Enum/UserFriendCategory` "NewEnumerator3")) (== Category (enumliteral `/Xsolla/Login/Enum/UserFriendCategory` "NewEnumerator4")))))

(fn `Init`
  (params (InDemo :type "/Xsolla/Login/Interface/BPI_Demo Interface") (InDemoWidget :type "/Xsolla/Login/Interface/BPI_DemoWidget Interface"))
  (set `self.Demo` InDemo)
  (set `self.DemoWidget` InDemoWidget))

(fn `IsValidFriendRecommendation`
  (params (Category :type "/Xsolla/Login/Enum/UserFriendCategory Enum" :default "NewEnumerator0"))
  (returns (IsValid :type Boolean))
  (return (or (`|EnumEquality` Category "NewEnumerator5") (`|EnumEquality` Category "NewEnumerator1") (`|EnumEquality` Category "NewEnumerator2"))))

(fn `ResetFriendsRequestsFlags`
  (set `self.FriendsRequestsReady` (`|MakeMap` "friends" false "friend_requested" false "friend_requested_by" false "blocked" :!type "EXsollaFriendsType Enum")))

(fn `ShowLoginError`
  (params (code :type String) (description :type String))
  (`/Xsolla/Common/BP_DemoUtils.ShowLoginError` code description))

(fn `UpdateProperIconPresenters`
  (params (IconPresenters :type "Array of /Xsolla/Common/Interface/BPI_IconPresenter Interface") (ImageURL :type String) (Icon :type "SlateBrush Structure") (IsErro :type Boolean))
  (for _array_element IconPresenters
    (bind _imageurl (`/Xsolla/Common/Interface/BPI_IconPresenter.GetImageUrl` _array_element))
    (if (`KismetStringLibrary.EqualEqual_StrStr` _imageurl ImageURL)
      (`/Xsolla/Common/Interface/BPI_IconPresenter.RefreshIcon` _array_element (select `bool` IsErro :`false` Icon :`true` (`WidgetBlueprintLibrary.MakeBrushFromTexture` "/Xsolla/Common/Assets/Icon/T_Icon_NotLoaded.T_Icon_NotLoaded" 100 100))))))

(fn `UserActionRequiresConfirmation`
  (params (Action :type Byte))
  (returns (RequiresConfirmation :type Boolean))
  (return (or (== Action (enumliteral `/Xsolla/Login/Enum/UserActionType` "NewEnumerator6")) (== Action (enumliteral `/Xsolla/Login/Enum/UserActionType` "NewEnumerator2")))))