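; Login controller for the Xsolla demo that runs registration, password reset and all sign-in flows through XsollaLoginSubsystem.
; Each flow toggles a loader; most errors open LoginWidget popups, while successful logins reach HandleSuccessfulAuthentication, which opens the store demo or prints the token.
; Social login uses native auth on Android when allowed, otherwise a browser.
; Phone and email login can auto-poll for confirmation codes, matched by operation ID, with limited retries.
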(event `self.RegisterUser`
  (params (Username :type String) (Password :type String) (Email :type String) (LoginWidget :type "/Xsolla/Login/Interface/BPI_LoginWidget Interface"))
  ;[1 1 1] Registration
  (`/Xsolla/Common/BP_DemoUtils.ShowLoader` true)
  (if (`XsollaLoginLibrary.IsEmailValid` Email)
    (`XsollaLoginSubsystem.RegisterUser` :`self` (subsystem `XsollaLoginSubsystem`) :`Username` Username :`Password` Password :`Email` Email :`State` "xsollatest" :`SuccessCallback` (delegate `OnRegistrationSuccess`) :`ErrorCallback` (delegate `OnRegistrationError`))
    (else
      (`/Xsolla/Common/BP_DemoUtils.ShowLoader` false)
      (`/Xsolla/Login/Interface/BPI_LoginWidget.ShowPopup` LoginWidget "" (`KismetTextLibrary.Conv_TextToString` (`|FormatText` "Invalid email")) true))))

(event `self.AuthenticateViaSessionTicket`
  (params (Provider :type String) (SessionTicket :type String) (Code :type String) (AppId :type String) (LoginWidget :type "/Xsolla/Login/Interface/BPI_LoginWidget Interface"))
  ;[1 1 1] Auth via session ticket
  (`/Xsolla/Common/BP_DemoUtils.ShowLoader` true)
  (`XsollaLoginSubsystem.AuthenticateWithSessionTicket` (subsystem `XsollaLoginSubsystem`) Provider SessionTicket Code AppId "xsollatest" "" (delegate `OnCrossAuthComplete`) (delegate `OnCrossAuthError`)))

(event `self.AuthenticateUser`
  (params (Username :type String) (Password :type String) (RememberMe :type Boolean) (LoginWidget :type "/Xsolla/Login/Interface/BPI_LoginWidget Interface"))
  ;[1 1 1] Basic auth
  (`/Xsolla/Common/BP_DemoUtils.ShowLoader` true)
  (`XsollaLoginSubsystem.AuthenticateUser` (subsystem `XsollaLoginSubsystem`) Username Password "" (delegate `OnAuthenticationSucces`) (delegate `OnAuthenticationError`) RememberMe))

(event `self.AuthenticateViaAccessToken`
  (params (Email :type String) (LoginWidget :type "/Xsolla/Login/Interface/BPI_LoginWidget Interface"))
  ;[1 1 1] Custom auth
  (`/Xsolla/Common/BP_DemoUtils.ShowLoader` true)
  (`XsollaLoginSubsystem.GetAccessTokenFromCustomAuthServer` (subsystem `XsollaLoginSubsystem`) (make `XsollaParameters` (`|MakeMap` "email" (`XsollaUtilsLibrary.Conv_StringToXsollaJsonVariant` Email))) (delegate `OnAuthViaAccessTokenSuccess`) (delegate `OnAuthViaAccessTokenFailed`)))

(event `OnAuthenticationSucces`
  (params (LoginData :type "XsollaLoginData Structure (by ref)"))
  ;[1 1 1] Basic auth
  (`/Xsolla/Common/BP_DemoUtils.ShowLoader` false)
  (`self.HandleSuccessfulAuthentication` LoginData (stale `self.AuthenticateUser` LoginWidget)))

(event `OnCrossAuthComplete`
  (params (LoginData :type "XsollaLoginData Structure (by ref)"))
  ;[1 1 1] Auth via session ticket
  (`/Xsolla/Common/BP_DemoUtils.ShowLoader` false)
  (`self.HandleSuccessfulAuthentication` LoginData (stale `self.AuthenticateViaSessionTicket` LoginWidget)))

(event `OnAuthViaAccessTokenSuccess`
  (params (AccessToken :type String))
  ;[1 1 1] Custom auth
  (`/Xsolla/Common/BP_DemoUtils.ShowLoader` false)
  (`XsollaLoginSubsystem.SetToken` (subsystem `XsollaLoginSubsystem`) AccessToken)
  (`self.HandleSuccessfulAuthentication` (`XsollaLoginSubsystem.GetLoginData` (subsystem `XsollaLoginSubsystem`)) (stale `self.AuthenticateViaAccessToken` LoginWidget)))

(event `OnRegistrationSuccess`
  (params (LoginData :type "XsollaLoginData Structure (by ref)"))
  ;[1 1 1] Registration
  (`/Xsolla/Common/BP_DemoUtils.ShowLoader` false)
  (if (`KismetStringLibrary.IsEmpty` (`.JWT` (break `XsollaAuthToken` (`.AuthToken` (break `XsollaLoginData` LoginData)))))
    (`/Xsolla/Login/Interface/BPI_LoginWidget.ShowPopup` (stale `self.RegisterUser` LoginWidget) (`KismetTextLibrary.Conv_TextToString` (`|FormatText` "Account successfully created")) (`KismetTextLibrary.Conv_TextToString` (`|FormatText` "Confirm your email address using the instructions we sent to {email}." (stale `self.RegisterUser` Email))) false)
    (else
      (`self.HandleSuccessfulAuthentication` LoginData (stale `self.RegisterUser` LoginWidget)))))

(event `OnAuthenticationError`
  (params (Code :type String) (Description :type String))
  ;[1 1 1] Basic auth
  (`/Xsolla/Common/BP_DemoUtils.ShowLoader` false)
  (`/Xsolla/Login/Interface/BPI_LoginWidget.ShowPopup` (stale `self.AuthenticateUser` LoginWidget) "" Description true))

(event `OnCrossAuthError`
  (params (Code :type String) (Description :type String))
  ;[1 1 1] Auth via session ticket
  (`/Xsolla/Common/BP_DemoUtils.ShowLoader` false))

(event `OnAuthViaAccessTokenFailed`
  (params (Code :type String) (Description :type String))
  ;[1 1 1] Custom auth
  (`/Xsolla/Common/BP_DemoUtils.ShowLoader` false)
  (`/Xsolla/Login/Interface/BPI_LoginWidget.ShowPopup` (stale `self.AuthenticateViaAccessToken` LoginWidget) Code Description true))

(event `OnRegistrationError`
  (params (Code :type String) (Description :type String))
  ;[1 1 1] Registration
  (`/Xsolla/Common/BP_DemoUtils.ShowLoader` false)
  (`/Xsolla/Login/Interface/BPI_LoginWidget.ShowPopup` (stale `self.RegisterUser` LoginWidget) "" Description true))

(event `self.AuthenticateViaSocialNetwork`
  (params (Provider :type String) (LoginWidget :type "/Xsolla/Login/Interface/BPI_LoginWidget Interface"))
  ;[1 1 1] Auth via social networks
  (if (and (`XsollaLoginSettings.bAllowNativeAuth` (`XsollaLoginLibrary.GetLoginSettings`)) (`KismetStringLibrary.EqualEqual_StrStr` (`GameplayStatics.GetPlatformName`) "Android"))
    (`self.AuthenticateViaSocialNetworkNative` Provider LoginWidget)
    (else
      (`self.AuthenticateViaSocialNetworkDesktop` Provider LoginWidget))))

(event `self.StartConfirmationCodePolling`
  (params (Option :type "/Xsolla/Login/Enum/LoginOption Enum" :default "NewEnumerator0") (LoginWidget :type "/Xsolla/Login/Interface/BPI_LoginWidget Interface"))
  ;[1 1 1] Auth confirmation code polling
  (if (`XsollaLoginSettings.SendPasswordlessAuthURL` (`XsollaLoginLibrary.GetLoginSettings`))
    (set `self.RemainingCodePollingAttempts` (`self.MaxCodePollingAttempts`))
    (`self.GetAuthenticationConfirmationCode` Option LoginWidget)))

(event `self.StartAuthenticationViaPhoneNumber`
  (params (PhoneNumber :type String) (LoginWidget :type "/Xsolla/Login/Interface/BPI_LoginWidget Interface"))
  ;[1 1 1] Phone number authentication
  (`/Xsolla/Common/BP_DemoUtils.ShowLoader` true)
  (`XsollaLoginSubsystem.StartAuthByPhoneNumber` (subsystem `XsollaLoginSubsystem`) PhoneNumber "" "xsollatest" (delegate `OnPhoneNumberAuthStartSuccess`) (delegate `OnPhoneNumberAuthStartError`)))

(event `self.StartAuthenticationViaEmail`
  (params (Email :type String) (LoginWidget :type "/Xsolla/Login/Interface/BPI_LoginWidget Interface"))
  ;[1 1 1] Email authentication
  (`/Xsolla/Common/BP_DemoUtils.ShowLoader` true)
  (`XsollaLoginSubsystem.StartAuthByEmail` (subsystem `XsollaLoginSubsystem`) Email "" "xsollatest" (delegate `OnEmailAuthStartSuccess`) (delegate `OnEmailAuthStartError`)))

(event `OnPhoneNumberAuthStartSuccess`
  (params (OperationId :type String))
  ;[1 1 1] Phone number authentication
  (`/Xsolla/Common/BP_DemoUtils.ShowLoader` false)
  (set `self.AuthOperationId` OperationId)
  (set `self.AuthUserId` (stale `self.StartAuthenticationViaPhoneNumber` PhoneNumber))
  (`/Xsolla/Login/Interface/BPI_LoginWidget.ShowAuthConfirmCodeScreen` (stale `self.StartAuthenticationViaPhoneNumber` LoginWidget))
  (`self.StartConfirmationCodePolling` "NewEnumerator0" (stale `self.StartAuthenticationViaPhoneNumber` LoginWidget)))

(event `OnEmailAuthStartSuccess`
  (params (OperationId :type String))
  ;[1 1 1] Email authentication
  (`/Xsolla/Common/BP_DemoUtils.ShowLoader` false)
  (set `self.AuthOperationId` OperationId)
  (set `self.AuthUserId` (stale `self.StartAuthenticationViaEmail` Email))
  (`/Xsolla/Login/Interface/BPI_LoginWidget.ShowAuthConfirmCodeScreen` (stale `self.StartAuthenticationViaEmail` LoginWidget))
  (`self.StartConfirmationCodePolling` "NewEnumerator1" (stale `self.StartAuthenticationViaEmail` LoginWidget)))

(event `self.StopConfirmationCodePolling`
  ;[1 1 1] Auth confirmation code polling
  (set `self.AuthOperationId` ""))

(event `OnPhoneNumberAuthStartError`
  (params (Code :type String) (Description :type String))
  ;[1 1 1] Phone number authentication
  (`/Xsolla/Common/BP_DemoUtils.ShowLoader` false)
  (`/Xsolla/Login/Interface/BPI_LoginWidget.ShowPopup` (stale `self.StartAuthenticationViaPhoneNumber` LoginWidget) "" Description true))

(event `OnEmailAuthStartError`
  (params (Code :type String) (Description :type String))
  ;[1 1 1] Email authentication
  (`/Xsolla/Common/BP_DemoUtils.ShowLoader` false)
  (`/Xsolla/Login/Interface/BPI_LoginWidget.ShowPopup` (stale `self.StartAuthenticationViaEmail` LoginWidget) "" Description true))

(event `self.GetAuthenticationConfirmationCode`
  (params (Option :type "/Xsolla/Login/Enum/LoginOption Enum" :default "NewEnumerator0") (LoginWidget :type "/Xsolla/Login/Interface/BPI_LoginWidget Interface"))
  ;[1 1 1] Auth confirmation code polling
  (`XsollaLoginSubsystem.GetAuthConfirmationCode` :`self` (subsystem `XsollaLoginSubsystem`) :`UserId` (`self.AuthUserId`) :`OperationId` (`self.AuthOperationId`) :`SuccessCallback` (delegate `OnCodeReceived`) :`TimeoutCallback` (delegate `OnCodeTimeput`)))

(event `self.AuthenticateViaSocialNetworkNative`
  (params (Provider :type String) (LoginWidget :type "/Xsolla/Login/Interface/BPI_LoginWidget Interface"))
  ;[1 1 1] Auth via social networks
  (`XsollaLoginSubsystem.LaunchNativeSocialAuthentication` (subsystem `XsollaLoginSubsystem`) Provider (delegate `OnNativeAuthSuccess`) (delegate `OnNativeAuthCancelled`) (delegate `OnNativeAuthError`) true))

(event `OnCodeReceived`
  (params (Code :type String) (OperationId :type String))
  (bind _authuserid (`self.AuthUserId`))
  ;[1 1 1] Auth confirmation code polling
  (if (`KismetStringLibrary.EqualEqual_StrStr` OperationId (`self.AuthOperationId`))
    (switch `/Xsolla/Login/Enum/LoginOption` (stale `self.GetAuthenticationConfirmationCode` Option)
      (:`NewEnumerator0`
        (`self.CompleteAuthenticationViaPhoneNumber` Code _authuserid (stale `self.GetAuthenticationConfirmationCode` LoginWidget)))
      (:`NewEnumerator1`
        (`self.CompleteAuthenticationViaEmail` Code _authuserid (stale `self.GetAuthenticationConfirmationCode` LoginWidget))))))

(event `OnNativeAuthSuccess`
  (params (LoginData :type "XsollaLoginData Structure (by ref)"))
  ;[1 1 1] Auth via social networks
  (`XsollaLoginSubsystem.SetLoginData` (subsystem `XsollaLoginSubsystem`) LoginData true)
  (`self.HandleSuccessfulAuthentication` LoginData (stale `self.AuthenticateViaSocialNetworkNative` LoginWidget)))

(event `self.CompleteAuthenticationViaPhoneNumber`
  (params (Code :type String) (PhoneNumber :type String) (LoginWidget :type "/Xsolla/Login/Interface/BPI_LoginWidget Interface"))
  ;[1 1 1] Phone number authentication
  (`/Xsolla/Common/BP_DemoUtils.ShowLoader` true)
  (`XsollaLoginSubsystem.CompleteAuthByPhoneNumber` (subsystem `XsollaLoginSubsystem`) Code (`self.AuthOperationId`) PhoneNumber (delegate `OnPhoneNumberAuthCompleteSuccess`) (delegate `OnPhoneNumberAuthCompleteError]`)))

(event `self.CompleteAuthenticationViaEmail`
  (params (Code :type String) (Email :type String) (LoginWidget :type "/Xsolla/Login/Interface/BPI_LoginWidget Interface"))
  ;[1 1 1] Email authentication
  (`/Xsolla/Common/BP_DemoUtils.ShowLoader` true)
  (`XsollaLoginSubsystem.CompleteAuthByEmail` (subsystem `XsollaLoginSubsystem`) Code (`self.AuthOperationId`) Email (delegate `OnEmailAuthCompleteSuccess`) (delegate `OnEmailAuthCompleteError]`)))

(event `OnNativeAuthCancelled`
  ;[1 1 1] Auth via social networks
)

(event `OnNativeAuthError`
  (params (Code :type String) (Description :type String))
  ;[1 1 1] Auth via social networks
  (`/Xsolla/Common/BP_DemoUtils.ShowLoader` false)
  (`/Xsolla/Login/Interface/BPI_LoginWidget.ShowPopup` (stale `self.AuthenticateViaSocialNetworkNative` LoginWidget) "" Description true))

(event `OnCodeTimeput`
  (params (OperationId :type String))
  ;[1 1 1] Auth confirmation code polling
  (if (and (`KismetStringLibrary.EqualEqual_StrStr` OperationId (`self.AuthOperationId`)) (> (`self.RemainingCodePollingAttempts`) 0))
    (set `self.RemainingCodePollingAttempts` (- (`self.RemainingCodePollingAttempts`) 1))
    (`self.GetAuthenticationConfirmationCode` (stale `self.GetAuthenticationConfirmationCode` Option) (stale `self.GetAuthenticationConfirmationCode` LoginWidget))))

(event `OnPhoneNumberAuthCompleteSuccess`
  (params (LoginData :type "XsollaLoginData Structure (by ref)"))
  ;[1 1 1] Phone number authentication
  (`self.StopConfirmationCodePolling`)
  (`/Xsolla/Common/BP_DemoUtils.ShowLoader` false)
  (`self.HandleSuccessfulAuthentication` LoginData (stale `self.CompleteAuthenticationViaPhoneNumber` LoginWidget)))

(event `OnEmailAuthCompleteSuccess`
  (params (LoginData :type "XsollaLoginData Structure (by ref)"))
  ;[1 1 1] Email authentication
  (`self.StopConfirmationCodePolling`)
  (`/Xsolla/Common/BP_DemoUtils.ShowLoader` false)
  (`self.HandleSuccessfulAuthentication` LoginData (stale `self.CompleteAuthenticationViaEmail` LoginWidget)))

(event `OnPhoneNumberAuthCompleteError]`
  (params (Code :type String) (Description :type String))
  ;[1 1 1] Phone number authentication
  (`/Xsolla/Common/BP_DemoUtils.ShowLoader` false)
  (`/Xsolla/Login/Interface/BPI_LoginWidget.ShowPopup` (stale `self.CompleteAuthenticationViaPhoneNumber` LoginWidget) "" Description true))

(event `OnEmailAuthCompleteError]`
  (params (Code :type String) (Description :type String))
  ;[1 1 1] Email authentication
  (`/Xsolla/Common/BP_DemoUtils.ShowLoader` false)
  (`/Xsolla/Login/Interface/BPI_LoginWidget.ShowPopup` (stale `self.CompleteAuthenticationViaEmail` LoginWidget) "" Description true))

(event `self.AuthenticateViaSocialNetworkDesktop`
  (params (Provider :type String) (WidgetLogin :type "/Xsolla/Login/Interface/BPI_LoginWidget Interface"))
  ;[1 1 1] Auth via social networks
  (`/Xsolla/Common/BP_DemoUtils.ShowLoader` true)
  (`XsollaLoginSubsystem.GetSocialAuthenticationUrl` :`self` (subsystem `XsollaLoginSubsystem`) :`ProviderName` Provider :`State` "xsollatest" :`SuccessCallback` (delegate `OnSocialAuthUrlReceived`) :`ErrorCallback` (delegate `OnSocialAuthError`)))

(event `OnSocialAuthUrlReceived`
  (params (Url :type String))
  ;[1 1 1] Auth via social networks
  (`/Xsolla/Common/BP_DemoUtils.ShowLoader` false)
  (bind _browserwidget (`XsollaLoginSubsystem.LaunchSocialAuthentication` (subsystem `XsollaLoginSubsystem`) Url true))
  (bind _asw_login_browser (cast `/Xsolla/Login/Components/W_LoginBrowser` _browserwidget))
  (add `/Xsolla/Login/Components/W_LoginBrowser.Browser Closed` _asw_login_browser (delegate `OnSocialAuthenticationCompleted`)))

(event `OnSocialAuthenticationCompleted`
  (params (`Authentication Completed` :type Boolean))
  ;[1 1 1] Auth via social networks
  (if `Authentication Completed`
    (`self.HandleSuccessfulAuthentication` (`XsollaLoginSubsystem.GetLoginData` (subsystem `XsollaLoginSubsystem`)) (stale `self.AuthenticateViaSocialNetworkDesktop` WidgetLogin))))

(event `OnSocialAuthError`
  (params (Code :type String) (Description :type String))
  ;[1 1 1] Auth via social networks
  (`/Xsolla/Common/BP_DemoUtils.ShowLoader` false)
  (`/Xsolla/Login/Interface/BPI_LoginWidget.ShowPopup` (stale `self.AuthenticateViaSocialNetworkDesktop` WidgetLogin) "" Description true))

(event `self.AuthenticatePlatformAccount`
  (params (LoginWidget :type "/Xsolla/Login/Interface/BPI_LoginWidget Interface"))
  (bind _returnvalue (`XsollaLoginLibrary.GetLoginSettings`))
  ;[1 1 1] Auth with platform account
  (`/Xsolla/Common/BP_DemoUtils.ShowLoader` true)
  (`XsollaLoginSubsystem.AuthenticatePlatformAccountUser` (subsystem `XsollaLoginSubsystem`) (`XsollaLoginSettings.PlatformAccountID` _returnvalue) (`XsollaLoginSettings.Platform` _returnvalue) (delegate `OnPlatformAuthCompleted`) (delegate `OnPlatformAuthError`)))

(event `self.ResetPassword`
  (params (User :type String) (LoginWidget :type "/Xsolla/Login/Interface/BPI_LoginWidget Interface"))
  ;[1 1 1] Password reset
  (`/Xsolla/Common/BP_DemoUtils.ShowLoader` true)
  (`XsollaLoginSubsystem.ResetUserPassword` (subsystem `XsollaLoginSubsystem`) User (delegate `OnResetPasswordSuccess`) (delegate `OnResetPasswordError`)))

(event `OnResetPasswordSuccess`
  ;[1 1 1] Password reset
  (`/Xsolla/Common/BP_DemoUtils.ShowLoader` false)
  (`/Xsolla/Login/Interface/BPI_LoginWidget.ShowPopup` (stale `self.ResetPassword` LoginWidget) (`KismetTextLibrary.Conv_TextToString` (`|FormatText` "Confirm password reset")) (`KismetTextLibrary.Conv_TextToString` (`|FormatText` "Change your password using the instructions we sent to your email.")) false))

(event `OnPlatformAuthCompleted`
  (params (LoginData :type "XsollaLoginData Structure (by ref)"))
  ;[1 1 1] Auth with platform account
  (`/Xsolla/Common/BP_DemoUtils.ShowLoader` false)
  (`self.HandleSuccessfulAuthentication` LoginData (stale `self.AuthenticatePlatformAccount` LoginWidget)))

(event `OnResetPasswordError`
  (params (Code :type String) (Description :type String))
  ;[1 1 1] Password reset
  (`/Xsolla/Common/BP_DemoUtils.ShowLoader` false)
  (`/Xsolla/Login/Interface/BPI_LoginWidget.ShowPopup` (stale `self.ResetPassword` LoginWidget) "" Description true))

(event `OnPlatformAuthError`
  (params (Code :type String) (Description :type String))
  ;[1 1 1] Auth with platform account
  (`/Xsolla/Common/BP_DemoUtils.ShowLoader` false)
  (`/Xsolla/Login/Interface/BPI_LoginWidget.ShowPopup` (stale `self.AuthenticatePlatformAccount` LoginWidget) "" Description true))

(event `self.ValidateToken`
  (params (LoginWidget :type "/Xsolla/Login/Interface/BPI_LoginWidget Interface"))
  ;[1 1 1] Validate cached token
  (`/Xsolla/Common/BP_DemoUtils.ShowLoader` true)
  (`XsollaLoginSubsystem.ValidateToken` (subsystem `XsollaLoginSubsystem`) (delegate `OnValidationTokenSuccess`) (delegate `OnValidationTokenError`)))

(event `self.RefreshToken`
  (params (RefreshToken :type String) (LoginWidget :type "/Xsolla/Login/Interface/BPI_LoginWidget Interface"))
  ;[1 1 1] Refresh user token (OAuth 2.0 only)
  (`/Xsolla/Common/BP_DemoUtils.ShowLoader` true)
  (`XsollaLoginSubsystem.RefreshToken` (subsystem `XsollaLoginSubsystem`) RefreshToken (delegate `OnRefreshTokenSuccess`) (delegate `OnRefreshTokenError`)))

(event `OnValidationTokenSuccess`
  (params (LoginData :type "XsollaLoginData Structure (by ref)"))
  ;[1 1 1] Validate cached token
  (`/Xsolla/Common/BP_DemoUtils.ShowLoader` false)
  (`self.HandleSuccessfulAuthentication` LoginData (stale `self.ValidateToken` LoginWidget)))

(event `OnRefreshTokenSuccess`
  (params (LoginData :type "XsollaLoginData Structure (by ref)"))
  ;[1 1 1] Refresh user token (OAuth 2.0 only)
  (`/Xsolla/Common/BP_DemoUtils.ShowLoader` false)
  (`self.HandleSuccessfulAuthentication` LoginData (stale `self.RefreshToken` LoginWidget)))

(event `OnValidationTokenError`
  (params (Code :type String) (Description :type String))
  ;[1 1 1] Validate cached token
  (`/Xsolla/Common/BP_DemoUtils.ShowLoader` false))

(event `OnRefreshTokenError`
  (params (Code :type String) (Description :type String))
  ;[1 1 1] Refresh user token (OAuth 2.0 only)
  (`/Xsolla/Common/BP_DemoUtils.ShowLoader` false))

(fn `HandleSuccessfulAuthentication`
  (params (LoginData :type "XsollaLoginData Structure") (LoginWidget :type "/Xsolla/Login/Interface/BPI_LoginWidget Interface"))
  (bind _asxsolla_demo_game_mode_base (cast `/Xsolla/Common/XsollaDemoGameModeBase` (`GameplayStatics.GetGameMode` self)))
  (bind _returnvalue (`XsollaDemoGameModeBase.GetStoreDemo` _asxsolla_demo_game_mode_base))
  (if (`KismetSystemLibrary.IsValidClass` _returnvalue)
    (bind _returnvalue_2 (`|CreateWidget` _returnvalue))
    (`UserWidget.AddToPlayerScreen` _returnvalue_2 0)
    (`/Xsolla/Login/Interface/BPI_LoginWidget.Destroy` LoginWidget)
    (else
      (`KismetSystemLibrary.PrintString` (break `XsollaAuthToken` (`.AuthToken` (break `XsollaLoginData` LoginData)))))))