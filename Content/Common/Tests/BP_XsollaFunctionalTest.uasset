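; BP_XsollaFunctionalTest is a functional test Blueprint for Xsolla that handles common setup and cleanup.
; PrepareTest warns about leftover top-level widgets, restores default settings, sets up the test playground, creates the login widget and sets the IsReady flag.
; StartTest binds a finish handler, which unbinds itself and removes all top-level user widgets when the test ends.
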(event `self.ReceivePrepareTest`
  (bind _foundwidgets (`WidgetBlueprintLibrary.GetAllWidgetsOfClass` "/Script/UMG.UserWidget"))
  (if (> (`KismetArrayLibrary.Array_Length` _foundwidgets) 0)
    (`self.AddWarning` "Some widgets were not destroyed properly"))
  (`self.SetupProjectSettings`)
  (`TestHelper.SetupTestPlayground`)
  (`TestHelper.CreateLoginWidget`)
  (set `self.bIsReady` true))

(event `self.ReceiveStartTest`
  (add `self.OnTestFinished` (delegate `TestFinishedEvent`)))

(event `TestFinishedEvent`
  (remove `self.OnTestFinished` (delegate `TestFinishedEvent`))
  (bind _foundwidgets (`WidgetBlueprintLibrary.GetAllWidgetsOfClass` "/Script/UMG.UserWidget"))
  (for _array_element _foundwidgets
    (`Widget.RemoveFromParent` _array_element)))

(fn `IsReady`
  (returns (ReturnValue :type Boolean))
  (return (`self.bIsReady`)))

(fn `SetupProjectSettings`
  (`TestHelper.RestoreDefaultSettings`))

(fn `UserConstructionScript`)