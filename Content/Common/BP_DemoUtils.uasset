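; Blueprint utility library for the Xsolla demo, providing shared UI, link and dev-menu settings helpers.
; It looks up links by type in a data table and shows or clears loading screens and message popups, including login errors.
; Dev-menu data persists in a save slot, falling back to project settings when absent.
; The web shop URL combines the saved or default store URL with the current login token.
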(fn `Does Dev Menu Save Game Exist`
  (returns (bIsExist :type Boolean))
  (locals (DevMenuSaveSlot :type String :default "XsollaDevMenuSaveSlot"))
  (bind _returnvalue (`GameplayStatics.DoesSaveGameExist` (`local.DevMenuSaveSlot`)))
  (return _returnvalue))

(fn `GetWebShopUrlWithToken`
  (returns (Url :type String))
  (bind _webstoreurl (`XsollaProjectSettings.WebStoreURL` (`XsollaSettingsLibrary.GetProjectSettings`)))
  (bind ((`WebStoreUrl_19_E93CD4704454267B34E50FB235664FB6` _webstoreurl_2)) (break `/Xsolla/Common/Misc/XsollaDevMenuData` (`self.LoadDevMenuData` (`local.__WorldContext`))))
  (bind _returnvalue (select `bool` (`self.Does Dev Menu Save Game Exist` (`local.__WorldContext`)) :`false` _webstoreurl :`true` (select `bool` (not (`KismetStringLibrary.IsEmpty` _webstoreurl_2)) :`false` _webstoreurl :`true` _webstoreurl_2)))
  (return (`KismetTextLibrary.Conv_TextToString` (`|FormatText` "{WebStoreUrl}{ParameterSymbol}token={Token}&remember_me=false" _returnvalue (select `bool` (`KismetStringLibrary.Contains` _returnvalue "?") :`false` "?" :`true` "&") (`.JWT` (break `XsollaAuthToken` (`.AuthToken` (break `XsollaLoginData` (`XsollaLoginSubsystem.GetLoginData` (subsystem `XsollaLoginSubsystem`))))))))))

(fn `GetXsollaLink`
  (params (LinkType :type "/Xsolla/Common/Misc/Links/XsollaLinkType Enum" :default "NewEnumerator0"))
  (returns (Link :type String))
  (bind _outrownames (`DataTableFunctionLibrary.GetDataTableRowNames` "/Xsolla/Common/Misc/Links/DT_XsollaLinks.DT_XsollaLinks"))
  (for _array_element _outrownames
    (bind _returnvalue (`|GetDataTableRow` "/Xsolla/Common/Misc/Links/DT_XsollaLinks.DT_XsollaLinks" _array_element)
      (:`then`
        (bind (_linktype _link) (break `/Xsolla/Common/Misc/Links/S_XsollaLink` _returnvalue))
        (if (`|EnumEquality` _linktype LinkType)
          (return _link)))))
  (return "") ; Link with specified type wasn't found
)

(fn `LoadDevMenuData`
  (returns (DevMenuData :type "/Xsolla/Common/Misc/XsollaDevMenuData Structure"))
  (locals (DevMenuSaveSlot :type String :default "XsollaDevMenuSaveSlot"))
  (bind _returnvalue (`XsollaSettingsLibrary.GetProjectSettings`))
  (if (`self.Does Dev Menu Save Game Exist` (`local.__WorldContext`))
    (bind _returnvalue_2 (`GameplayStatics.LoadGameFromSlot` (`local.DevMenuSaveSlot`)))
    (bind _asxsolla_dev_menu_save_game (cast `/Xsolla/Common/Misc/XsollaDevMenuSaveGame` _returnvalue_2)
      (:`then`
        (return (`/Xsolla/Common/Misc/XsollaDevMenuSaveGame.DevMenuData` _asxsolla_dev_menu_save_game)))
      (:`CastFailed`
        _)))
  (return (make `/Xsolla/Common/Misc/XsollaDevMenuData` (`XsollaProjectSettings.LoginID` _returnvalue) (`XsollaProjectSettings.ProjectID` _returnvalue) (`XsollaProjectSettings.ClientID` _returnvalue) (`XsollaProjectSettings.WebStoreURL` _returnvalue))))

(fn `SaveDevMenuData`
  (params (DevMenuData :type "/Xsolla/Common/Misc/XsollaDevMenuData Structure"))
  (returns (IsSuccess :type Boolean))
  (locals (DevMenuSaveSlot :type String :default "XsollaDevMenuSaveSlot"))
  (bind _returnvalue (`GameplayStatics.LoadGameFromSlot` (`local.DevMenuSaveSlot`)))
  (bind _asxsolla_dev_menu_save_game (cast `/Xsolla/Common/Misc/XsollaDevMenuSaveGame` _returnvalue)
    (:`then`
      (set `/Xsolla/Common/Misc/XsollaDevMenuSaveGame.DevMenuData` DevMenuData _asxsolla_dev_menu_save_game)
      (bind _returnvalue_2 (`GameplayStatics.SaveGameToSlot` _asxsolla_dev_menu_save_game (`local.DevMenuSaveSlot`)))
      (return _returnvalue_2))
    (:`CastFailed`
      (bind _returnvalue_3 (`GameplayStatics.CreateSaveGameObject` "/Xsolla/Common/Misc/XsollaDevMenuSaveGame.XsollaDevMenuSaveGame_C"))
      (set `/Xsolla/Common/Misc/XsollaDevMenuSaveGame.DevMenuData` DevMenuData _returnvalue_3)
      (bind _returnvalue_4 (`GameplayStatics.SaveGameToSlot` _returnvalue_3 (`local.DevMenuSaveSlot`)))
      (return _returnvalue_4))))

(fn `ShowLoader`
  (params (ShowLoader :type Boolean))
  (if ShowLoader
    (bind _returnvalue (`|CreateWidget` "/Xsolla/Common/Components/Misc/W_LoadingScreen.W_LoadingScreen_C"))
    (`UserWidget.AddToViewport` _returnvalue 1)
    (else
      (bind _foundwidgets (`WidgetBlueprintLibrary.GetAllWidgetsOfClass` null "/Xsolla/Common/Components/Misc/W_LoadingScreen.W_LoadingScreen_C" false))
      (for _array_element _foundwidgets
        (`Widget.RemoveFromParent` _array_element)))))

(fn `ShowLoginError`
  (params (code :type String) (description :type String))
  (`self.ShowLoader` false)
  (`self.ShowMessagePopup` (`KismetTextLibrary.Conv_StringToText` description) true))

(fn `ShowMessagePopup`
  (params (message :type Text) (isError :type Boolean))
  (bind _returnvalue (`|CreateWidget` "/Xsolla/Common/Popup/W_MessagePopup.W_MessagePopup_C" null message isError))
  (`UserWidget.AddToViewport` _returnvalue 10000))